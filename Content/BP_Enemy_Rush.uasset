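; Rushing melee enemy that chases the top-down character once it enters the detection sphere.
; A self-repeating chase event uses AI MoveTo, then faces the player and briefly spawns a hitbox actor at the attack point.
; The loop retries failed moves and keeps polling while the target is out of range.
; Every hit taken asks the GameManager for a chance pickup and lowers health, destroying the enemy at zero.
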(event `self.ReceiveBeginPlay`
  (bind _returnvalue (`GameplayStatics.GetActorOfClass` "/Game/TopDown/Blueprints/BP_GameManager.BP_GameManager_C"))
  (set `self.Game Manager` _returnvalue))

(event `self.DetectionSphere.OnComponentBeginOverlap`
  (params (OverlappedComponent :type "PrimitiveComponent Object Reference") (OtherActor :type "Actor Object Reference") (OtherComp :type "PrimitiveComponent Object Reference") (OtherBodyIndex :type Integer) (bFromSweep :type Boolean) (SweepResult :type "HitResult Structure (by ref)"))
  (bind _asbp_top_down_character (cast `/Game/TopDown/Blueprints/BP_TopDownCharacter` OtherActor))
  (set `self.As BP Top Down Character` _asbp_top_down_character)
  (set `self.Active` true)
  (`self.ChasePlayer`))

(event `self.DetectionSphere.OnComponentEndOverlap`
  (params (OverlappedComponent :type "PrimitiveComponent Object Reference") (OtherActor :type "Actor Object Reference") (OtherComp :type "PrimitiveComponent Object Reference") (OtherBodyIndex :type Integer))
  (cast `/Game/TopDown/Blueprints/BP_TopDownCharacter` OtherActor)
  (set `self.Active` false))

(event `ChasePlayer`
  (bind (_returnvalue_location _returnvalue_rotation) (`KismetMathLibrary.BreakTransform` (`SceneComponent.K2_GetComponentToWorld` (`self.AttackSpawnPoint`))))
  (bind (_returnvalue_roll _returnvalue_pitch _returnvalue_yaw) (`KismetMathLibrary.BreakRotator` (`KismetMathLibrary.FindLookAtRotation` (`self.K2_GetActorLocation`) (`self.K2_GetActorLocation` (`GameplayStatics.GetPlayerCharacter` 0)))))
  (if (`self.Active`)
    (`AITask_MoveTo.AIMoveTo` (`AIBlueprintHelperLibrary.GetAIController` self) (0.0 0.0 0.0) (`self.As BP Top Down Character`) 5.0 "Enable" "Disable"
      (:`OnRequestFailed`
        (`KismetSystemLibrary.Delay` 1.0)
        (`self.ChasePlayer`))
      (:`OnMoveFinished`
        (`self.K2_SetActorRotation` (`KismetMathLibrary.MakeRotator` 0.0 0.0 _returnvalue_yaw))
        (`KismetSystemLibrary.Delay` 0.2)
        (bind _returnvalue (`|SpawnActorFromClass` "/Game/BP_Enemy_Rush_Hitbox.BP_Enemy_Rush_Hitbox_C" (`KismetMathLibrary.MakeTransform` _returnvalue_location _returnvalue_rotation) "Undefined" "MultiplyWithRoot" null null))
        (`KismetSystemLibrary.Delay` 0.4)
        (`self.K2_DestroyActor` _returnvalue)
        (`self.ChasePlayer`)))
    (else
      (`KismetSystemLibrary.Delay` 2.0)
      (`self.ChasePlayer`))))

(event `self.ReceiveAnyDamage`
  (params (Damage :type "Float (single-precision)") (DamageType :type "DamageType Object Reference") (InstigatedBy :type "Controller Object Reference") (DamageCauser :type "Actor Object Reference"))
  (`/Game/TopDown/Blueprints/BP_GameManager.SpawnPickup` (`self.Game Manager`) self 5)
  (bind _output_get (set `self.Health` (- (`self.Health`) (`KismetMathLibrary.Round` Damage))))
  (if (<= _output_get 0)
    (`self.K2_DestroyActor`)))

(fn `UserConstructionScript`)