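; Collector boss enemy that cycles through attack patterns and is destroyed when damage depletes its Health.
; Attacks opens with QuickShot fire at the player, then AttackCounter picks spin, log walls, burst fire, Lobber adds or bullet wall.
; Each pattern runs on a looping named timer, mostly rotating SpinTarget to place spawns.
; LoopAmount ends most patterns, advancing the counter and re-entering Attacks; BurstFire handles its own exit, returning to QuickShot between bursts.
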(event `self.ReceiveBeginPlay`
  (`self.Attacks`))

(event `Attacks`
  (`KismetSystemLibrary.Delay` 0.25)
  (`KismetSystemLibrary.K2_SetTimer` null "QuickShot" 0.33 true)
  (`KismetSystemLibrary.Delay` (`KismetMathLibrary.RandomFloatInRange` 0.8 1.1))
  (`KismetSystemLibrary.K2_ClearTimer` null "QuickShot")
  (`KismetSystemLibrary.Delay` 0.25)
  (switch `int` (`self.AttackCounter`)
    (:`Default`
      (set `self.AttackCounter` 0)
      (`self.Attacks`))
    (:`0`
      (`KismetSystemLibrary.K2_SetTimer` null "Spin" (`self.DelayBetweenBulletsSpin`) true))
    (:`1`
      (`KismetSystemLibrary.K2_SetTimer` null "LogWalls" (`self.DelayBetweenLogSpawn`) true))
    (:`2`
      (`KismetSystemLibrary.K2_SetTimer` null "BurstFire" (`self.DelayBetweenBurstFire`) true))
    (:`3`
      (`KismetSystemLibrary.K2_SetTimer` null "SpawnAdds" 0.75 true))
    (:`4`
      (`KismetSystemLibrary.K2_SetTimer` null "BulletWall" 0.05 true))))

(event `self.ReceiveAnyDamage`
  (params (Damage :type "Float (single-precision)") (DamageType :type "DamageType Object Reference") (InstigatedBy :type "Controller Object Reference") (DamageCauser :type "Actor Object Reference"))
  (bind _output_get (set `self.Health` (- (`self.Health`) (`KismetMathLibrary.Round` Damage))))
  (if (<= _output_get 0)
    (`self.K2_DestroyActor`)))

(fn `BulletWall`
  (bind _index (`self.Index`))
  (bind _returnvalue_location (`KismetMathLibrary.BreakTransform` (`SceneComponent.K2_GetComponentToWorld` (`self.BulletSpawnPoint`))))
  (for _index_2 (range 4)
    (`SceneComponent.K2_SetWorldRotation` (`self.SpinTarget`) (`KismetMathLibrary.MakeRotator` 0.0 0.0 (`KismetMathLibrary.Conv_IntToDouble` (* _index_2 90))) false false)
    (`|SpawnActorFromClass` "/Game/BP_Enemy_Projectile_Collector_Boss_Wall.BP_Enemy_Projectile_Collector_Boss_Wall_C" (`KismetMathLibrary.MakeTransform` _returnvalue_location) "Undefined" "MultiplyWithRoot" null null))
  (`SceneComponent.K2_SetRelativeRotation` :`self` (`self.SpinTarget`))
  (`SceneComponent.K2_SetRelativeLocation` (`self.BulletSpawnPoint`) (`KismetMathLibrary.MakeVector` (`KismetMathLibrary.Conv_IntToDouble` (+ (* _index 25) 75)) 0.0 -45.0) false false)
  (bind _result (`/Engine/EditorBlueprintResources/StandardMacros.IncrementInt` _index)
    (:`  `
      (if (>= _result 25)
        (`SceneComponent.K2_SetRelativeLocation` (`self.BulletSpawnPoint`) (75.0 0.0 -45.0) false false)
        (`self.LoopAmount` 25 "BulletWall")))))

(fn `BurstFire`
  (bind (_returnvalue_location _returnvalue_rotation) (`KismetMathLibrary.BreakTransform` (`SceneComponent.K2_GetComponentToWorld` (`self.BulletSpawnPoint`))))
  (bind (_returnvalue_roll _returnvalue_pitch _returnvalue_yaw) (`KismetMathLibrary.BreakRotator` (`KismetMathLibrary.FindLookAtRotation` (`self.K2_GetActorLocation`) (`self.K2_GetActorLocation` (`GameplayStatics.GetPlayerCharacter` 0)))))
  (`/Engine/EditorBlueprintResources/StandardMacros.IncrementInt` (`self.Index`)
    (:`  `
      (`SceneComponent.K2_SetRelativeRotation` (`self.SpinTarget`) (`KismetMathLibrary.MakeRotator` 0.0 0.0 _returnvalue_yaw) false false)
      (for _index (range -2 3)
        (bind _returnvalue (`|SpawnActorFromClass` "/Game/BP_Enemy_Projectile_Collector_Boss_Burst.BP_Enemy_Projectile_Collector_Boss_Burst_C" (`KismetMathLibrary.MakeTransform` _returnvalue_location _returnvalue_rotation) "Undefined" "MultiplyWithRoot" null null))
        (`ProjectileMovementComponent.SetVelocityInLocalSpace` (`/Game/BP_Enemy_Projectile_Collector_Boss_Burst.ProjectileMovement` _returnvalue) (`KismetMathLibrary.MakeVector` 1600.0 (* _index 75))))
      (if (== (`KismetMathLibrary.FMod` (`KismetMathLibrary.Conv_IntToDouble` (`self.Index`)) 5.0) 0.0)
        (`KismetSystemLibrary.K2_ClearTimer` null "BurstFire")
        (if (== (`self.Index`) 15)
          (set `self.Index` 0)
          (`/Engine/EditorBlueprintResources/StandardMacros.IncrementInt` (`self.AttackCounter`)
            (:`  `
              _)))
        (`self.Attacks`)))))

(fn `LogWalls`
  (bind (_returnvalue_roll _returnvalue_pitch) (`KismetMathLibrary.BreakRotator` (`SceneComponent.K2_GetComponentRotation` (`self.SpinTarget`))))
  (bind (_returnvalue_location _returnvalue_rotation) (`KismetMathLibrary.BreakTransform` (`SceneComponent.K2_GetComponentToWorld` (`self.LogSpawnPoint`))))
  (`/Engine/EditorBlueprintResources/StandardMacros.IncrementInt` (`self.Index`)
    (:`  `
      (`SceneComponent.K2_SetRelativeRotation` (`self.SpinTarget`) (`KismetMathLibrary.MakeRotator` _returnvalue_roll _returnvalue_pitch (`KismetMathLibrary.Conv_IntToDouble` (* (`self.Index`) 90))) false false)
      (`|SpawnActorFromClass` "/Game/TopDown/Blueprints/Greybox/BP_Enemy_Crafter_Log_Pile.BP_Enemy_Crafter_Log_Pile_C" (`KismetMathLibrary.MakeTransform` _returnvalue_location _returnvalue_rotation) "AdjustIfPossibleButAlwaysSpawn" "MultiplyWithRoot" null null)
      (`self.LoopAmount` 4 "LogWalls"))))

(fn `QuickShot`
  (bind (_returnvalue_location _returnvalue_rotation) (`KismetMathLibrary.BreakTransform` (`SceneComponent.K2_GetComponentToWorld` (`self.BulletSpawnPoint`))))
  (bind (_returnvalue_roll _returnvalue_pitch _returnvalue_yaw) (`KismetMathLibrary.BreakRotator` (`KismetMathLibrary.FindLookAtRotation` (`self.K2_GetActorLocation`) (`self.K2_GetActorLocation` (`GameplayStatics.GetPlayerCharacter` 0)))))
  (`SceneComponent.K2_SetRelativeRotation` (`self.SpinTarget`) (`KismetMathLibrary.MakeRotator` 0.0 0.0 _returnvalue_yaw) false false)
  (bind _returnvalue (`|SpawnActorFromClass` "/Game/BP_Enemy_Projectile_Collector_Boss_Burst.BP_Enemy_Projectile_Collector_Boss_Burst_C" (`KismetMathLibrary.MakeTransform` _returnvalue_location _returnvalue_rotation) "Undefined" "MultiplyWithRoot" null null))
  (bind _projectilemovement (`/Game/BP_Enemy_Projectile_Collector_Boss_Burst.ProjectileMovement` _returnvalue))
  (set `ProjectileMovementComponent.InitialSpeed` 1650.0 _projectilemovement)
  (set `ProjectileMovementComponent.MaxSpeed` 1650.0 _projectilemovement))

(fn `SpawnAdds`
  (bind _randomlocation (`NavigationSystemV1.K2_GetRandomReachablePointInRadius` (`self.K2_GetActorLocation`) 300.0 null null))
  (`/Engine/EditorBlueprintResources/StandardMacros.IncrementInt` (`self.Index`)
    (:`  `
      (set `self.Random Location` _randomlocation)
      (while (< (`KismetMathLibrary.Vector_Distance` (`self.K2_GetActorLocation` (`GameplayStatics.GetPlayerCharacter` 0)) (`self.Random Location`)) 100.0)
        (set `self.Random Location` _randomlocation))
      (`|SpawnActorFromClass` "/Game/BP_Enemy_Lobber.BP_Enemy_Lobber_C" (`KismetMathLibrary.MakeTransform` (`self.Random Location`)) "AdjustIfPossibleButDontSpawnIfColliding" "MultiplyWithRoot" null null)
      (`self.LoopAmount` 2 "SpawnAdds"))))

(fn `Spin`
  (bind (_returnvalue_location _returnvalue_rotation) (`KismetMathLibrary.BreakTransform` (`SceneComponent.K2_GetComponentToWorld` (`self.BulletSpawnPoint`))))
  (bind (_returnvalue_roll _returnvalue_pitch) (`KismetMathLibrary.BreakRotator` (`SceneComponent.K2_GetComponentRotation` (`self.SpinTarget`))))
  (`/Engine/EditorBlueprintResources/StandardMacros.IncrementInt` (`self.Index`)
    (:`  `
      (`SceneComponent.K2_SetRelativeRotation` (`self.SpinTarget`) (`KismetMathLibrary.MakeRotator` _returnvalue_roll _returnvalue_pitch (`KismetMathLibrary.Conv_IntToDouble` (* (`self.Index`) 12))) false false)
      (`|SpawnActorFromClass` "/Game/BP_Enemy_Projectile_Collector_Boss_Spin.BP_Enemy_Projectile_Collector_Boss_Spin_C" (`KismetMathLibrary.MakeTransform` _returnvalue_location _returnvalue_rotation) "Undefined" "MultiplyWithRoot" null null)
      (`self.LoopAmount` 90 "Spin"))))

(fn `UserConstructionScript`)