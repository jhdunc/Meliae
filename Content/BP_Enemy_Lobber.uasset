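; Ranged lobber enemy that repositions around the player and fires log projectiles.
; A self-restarting Move loop picks a reachable point away from the player, walks there, pauses, snaps to face the player, plays an attack montage and spawns the projectile.
; Damage spawns particles, rolls a pickup through BP_GameManager and lowers health until death, with the health bar updated on Tick.
; Touching the player deals contact damage and records the hit in game-instance stats.
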(event `self.ReceiveBeginPlay`
  (`self.Move`)
  (bind _returnvalue (`GameplayStatics.GetActorOfClass` "/Game/TopDown/Blueprints/BP_GameManager.BP_GameManager_C"))
  (set `self.GameManager` _returnvalue)
  (set `self.Health` (`self.MaxHealth`)))

(event `self.ReceiveTick`
  (params (DeltaSeconds :type "Float (single-precision)"))
  (`self.UpdateHealthbar`))

(event `self.ReceiveAnyDamage`
  (params (Damage :type "Float (single-precision)") (DamageType :type "DamageType Object Reference") (InstigatedBy :type "Controller Object Reference") (DamageCauser :type "Actor Object Reference"))
  (`NiagaraFunctionLibrary.SpawnSystemAtLocation` "/Game/GameFilesMeliae/VFX/DamageFlash/NG_EnemyDamageParticle.NG_EnemyDamageParticle" (`self.K2_GetActorLocation`))
  (`/Game/TopDown/Blueprints/BP_GameManager.SpawnPickup` (`self.GameManager`) self 5)
  (bind _output_get (set `self.Health` (- (`self.Health`) (`KismetMathLibrary.Round` Damage))))
  (if (<= _output_get 0)
    (`self.K2_DestroyActor`)))

(event `self.HitBox.OnComponentBeginOverlap`
  (params (OverlappedComponent :type "PrimitiveComponent Object Reference") (OtherActor :type "Actor Object Reference") (OtherComp :type "PrimitiveComponent Object Reference") (OtherBodyIndex :type Integer) (bFromSweep :type Boolean) (SweepResult :type "HitResult Structure (by ref)"))
  (cast `/Game/TopDown/Blueprints/BP_TopDownCharacter` OtherActor)
  (`GameplayStatics.ApplyDamage` OtherActor 1.0)
  (`self.ContactDamageStat`))

(event `Move`
  (bind _randomlocation (`NavigationSystemV1.K2_GetRandomReachablePointInRadius` (`self.K2_GetActorLocation`) 600.0 null null))
  (bind (_returnvalue_location _returnvalue_rotation) (`KismetMathLibrary.BreakTransform` (`SceneComponent.K2_GetComponentToWorld` (`self.BulletSpawnPoint`))))
  (set `self.Random Location` _randomlocation)
  (while (< (`KismetMathLibrary.Vector_Distance` (`self.K2_GetActorLocation` (`GameplayStatics.GetPlayerCharacter` 0)) (`self.Random Location`)) 450.0)
    (set `self.Random Location` _randomlocation))
  (`AITask_MoveTo.AIMoveTo` (`AIBlueprintHelperLibrary.GetAIController` self) (`self.Random Location`) null 10.0 "Enable" "Enable"
    (:`OnRequestFailed`
      (`self.Move`))
    (:`OnMoveFinished`
      (`KismetSystemLibrary.Delay` (`KismetMathLibrary.RandomFloatInRange` 1.4 1.55))
      (`self.K2_SetActorRotation` (`KismetMathLibrary.FindLookAtRotation` (`self.K2_GetActorLocation`) (`self.K2_GetActorLocation` (`GameplayStatics.GetPlayerCharacter` 0)))) ; Will need to make this gradual when its not a cube
      ;[0 0.000607 0.8469] Attack animation
      (`|PlayMontage` (`self.Mesh`) "/Game/GameFilesMeliae/Meshes/enemies/animations/AM_Carrier_Attack.AM_Carrier_Attack"
        (:`then`
          (`KismetSystemLibrary.Delay` (`KismetMathLibrary.RandomFloatInRange` 0.55 0.7))
          (`|SpawnActorFromClass` "/Game/BP_Enemy_Projectile_Lobber_Log.BP_Enemy_Projectile_Lobber_Log_C" (`KismetMathLibrary.MakeTransform` _returnvalue_location _returnvalue_rotation) "Undefined" "MultiplyWithRoot" null null)
          (`self.Move`))))))

(fn `UpdateHealthbar`
  (bind _aswb_enemy_health (cast `/Game/GameFilesMeliae/UI/WB_EnemyHealth` (`WidgetComponent.GetUserWidgetObject` (`self.HealthBarWidget`))))
  (set `/Game/GameFilesMeliae/UI/WB_EnemyHealth.Health` (/ (`self.Health`) (`self.MaxHealth`)) _aswb_enemy_health)
  (return))

(fn `UserConstructionScript`)