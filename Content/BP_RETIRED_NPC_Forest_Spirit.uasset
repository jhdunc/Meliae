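; Retired forest spirit NPC that continually turns to face the player's top-down character and moves toward it.
; On BeginPlay it caches the player character and starts a Rotate event that re-calls itself after short delays, interpolating yaw only toward the player.
; Tick adds movement input along its forward vector behind a short Delay.
; An unconnected SimpleMoveToLocation node never runs.
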(event `Rotate`
  (`self.K2_SetActorRotation` (`KismetMathLibrary.MakeRotator` 0.0 0.0 (.yaw (`KismetMathLibrary.RInterpTo` (`self.K2_GetActorRotation`) (`KismetMathLibrary.FindLookAtRotation` (`self.K2_GetActorLocation`) (`SceneComponent.K2_GetComponentLocation` (`Actor.RootComponent` (`self.As BP Top Down Character`)))) (`GameplayStatics.GetWorldDeltaSeconds`) 25.0))))
  (`KismetSystemLibrary.Delay` 0.01)
  (`self.Rotate`))

(event `self.ReceiveBeginPlay`
  (bind _asbp_top_down_character (cast `/Game/TopDown/Blueprints/BP_TopDownCharacter` (`GameplayStatics.GetPlayerCharacter` 0)))
  (set `self.As BP Top Down Character` _asbp_top_down_character)
  (`self.Rotate`))

(event `self.ReceiveTick`
  (params (DeltaSeconds :type "Float (single-precision)"))
  (`KismetSystemLibrary.Delay` 0.0125)
  (`self.AddMovementInput` (`KismetMathLibrary.GetForwardVector` (`self.K2_GetActorRotation`))))

(fn `UserConstructionScript`)