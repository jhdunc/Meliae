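; Heavy enemy that, while active, cycles through chasing the player, a shotgun attack and a timeline-driven rush toward the player.
; The shotgun fires two delayed pellet spreads from two muzzles, the second narrower and slower.
; A self-recalling Rotate event turns it toward the player, pausing from the first volley until the attack ends.
; It deals contact damage, updates the player's enemy counter, and can trigger pickup drops through the GameManager when hit.
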(event `Rotate`
  (if (not (`self.Rushing`))
    (`self.K2_SetActorRotation` (`KismetMathLibrary.MakeRotator` 0.0 0.0 (.yaw (`KismetMathLibrary.RInterpTo` (`self.K2_GetActorRotation`) (`KismetMathLibrary.FindLookAtRotation` (`self.K2_GetActorLocation`) (`self.K2_GetActorLocation` (`self.As BP Top Down Character`))) (`GameplayStatics.GetWorldDeltaSeconds`) 25.0)))))
  (`KismetSystemLibrary.Delay` 0.01)
  (`self.Rotate`))

(event `self.ReceiveDestroyed`
  (bind _as_bp_top_down_character (`self.As BP Top Down Character`))
  (set `/Game/TopDown/Blueprints/BP_TopDownCharacter.EnemyCounter` (- (`/Game/TopDown/Blueprints/BP_TopDownCharacter.EnemyCounter` _as_bp_top_down_character) 1) _as_bp_top_down_character))

(event `self.ReceiveBeginPlay`
  (bind _as_bp_top_down_character (`self.As BP Top Down Character`))
  (bind _asbp_top_down_character (cast `/Game/TopDown/Blueprints/BP_TopDownCharacter` (`GameplayStatics.GetPlayerCharacter` 0)))
  (set `self.As BP Top Down Character` _asbp_top_down_character)
  (`self.Loops`)
  (set `self.NumberOfPelletsTEMP` (`self.NumberOfPellets`))
  (`self.Rotate`)
  (bind _returnvalue (`GameplayStatics.GetActorOfClass` "/Game/TopDown/Blueprints/BP_GameManager.BP_GameManager_C"))
  (set `self.GameManager` _returnvalue)
  (set `/Game/TopDown/Blueprints/BP_TopDownCharacter.EnemyCounter` (+ (`/Game/TopDown/Blueprints/BP_TopDownCharacter.EnemyCounter` _as_bp_top_down_character) 1) _as_bp_top_down_character))

(event `self.ReceiveTick`
  (params (DeltaSeconds :type "Float (single-precision)")))

(event `Loops`
  (bind _attackcounter (`self.AttackCounter`))
  (if (`self.Active`)
    (switch `int` _attackcounter
      (:`Default`
        (set `self.AttackCounter` 0)
        (`self.Loops` :!label _label))
      (:`0`
        (`/Engine/EditorBlueprintResources/StandardMacros.IncrementInt` _attackcounter
          (:`  `
            (bind _asynctaskproxy (`AITask_MoveTo.AIMoveTo` (`AIBlueprintHelperLibrary.GetAIController` self) (0.0 0.0 0.0) (`GameplayStatics.GetPlayerCharacter` 0) -1.0 "Enable" "Enable" true false)
              (:`then`
                (`KismetSystemLibrary.Delay` (`KismetMathLibrary.RandomFloatInRange` 1.9 2.05))
                (`NavMovementComponent.StopActiveMovement` (`self.CharacterMovement`))
                (`CharacterMovementComponent.SetMovementMode` (`self.CharacterMovement`) "MOVE_Walking" 0)
                (goto _label))))))
      (:`1`
        (`/Engine/EditorBlueprintResources/StandardMacros.IncrementInt` _attackcounter
          (:`  `
            (set `self.MovementPaused` true)
            (`self.Shotgun`
              (:`End`
                (`|PlayMontage` (`self.Mesh`) "/Game/GameFilesMeliae/Meshes/enemies/animations/AM_Heavy_Attack.AM_Heavy_Attack"
                  (:`then`
                    (`KismetSystemLibrary.Delay` (`KismetMathLibrary.RandomFloatInRange` 0.45 0.6))
                    (set `self.Rushing` false)
                    (set `self.MovementPaused` false)
                    (goto _label))))))))
      (:`2`
        (`/Engine/EditorBlueprintResources/StandardMacros.IncrementInt` _attackcounter
          (:`  `
            (set `self.MovementPaused` true)
            (`KismetSystemLibrary.Delay` (`KismetMathLibrary.RandomFloatInRange` 0.9 1.05))
            (`|PlayMontage` (`self.Mesh`) "/Game/GameFilesMeliae/Meshes/enemies/animations/AM_Heavy_Swipe_Attack.AM_Heavy_Swipe_Attack"
              (:`then`
                (bind _location (`self.Rush`))
                (bind (_direction _newtrack_0) (`Timeline|Timeline` :!via `PlayFromStart`)
                  (:`Update`
                    (`self.K2_SetActorLocation` (`KismetMathLibrary.VLerp` (`self.K2_GetActorLocation`) _location _newtrack_0) true))
                  (:`Finished`
                    (set `self.MovementPaused` false)
                    (goto _label)))))))))
    (else
      (`KismetSystemLibrary.Delay` 0.2)
      (`self.Loops`))))

(event `self.Detection Radius.OnComponentBeginOverlap`
  (params (OverlappedComponent :type "PrimitiveComponent Object Reference") (OtherActor :type "Actor Object Reference") (OtherComp :type "PrimitiveComponent Object Reference") (OtherBodyIndex :type Integer) (bFromSweep :type Boolean) (SweepResult :type "HitResult Structure (by ref)")))

(event `self.Detection Radius.OnComponentEndOverlap`
  (params (OverlappedComponent :type "PrimitiveComponent Object Reference") (OtherActor :type "Actor Object Reference") (OtherComp :type "PrimitiveComponent Object Reference") (OtherBodyIndex :type Integer)))

(event `self.HitBox.OnComponentBeginOverlap`
  (params (OverlappedComponent :type "PrimitiveComponent Object Reference") (OtherActor :type "Actor Object Reference") (OtherComp :type "PrimitiveComponent Object Reference") (OtherBodyIndex :type Integer) (bFromSweep :type Boolean) (SweepResult :type "HitResult Structure (by ref)"))
  (bind _asbp_top_down_character (cast `/Game/TopDown/Blueprints/BP_TopDownCharacter` OtherActor))
  (`GameplayStatics.ApplyDamage` _asbp_top_down_character 1.0)
  (`self.ContactDamageStat`))

(event `self.ReceiveAnyDamage`
  (params (Damage :type "Float (single-precision)") (DamageType :type "DamageType Object Reference") (InstigatedBy :type "Controller Object Reference") (DamageCauser :type "Actor Object Reference"))
  (`NiagaraFunctionLibrary.SpawnSystemAtLocation` "/Game/GameFilesMeliae/VFX/DamageFlash/NG_EnemyDamageParticle.NG_EnemyDamageParticle" (`self.K2_GetActorLocation`) (struct) (1.1 1.1 1.1))
  (`/Game/TopDown/Blueprints/BP_GameManager.SpawnPickup` (`self.GameManager`) self 5)
  (bind _output_get (set `self.Health` (- (`self.Health`) (`KismetMathLibrary.Round` Damage))))
  (if (<= _output_get 0)
    (`self.K2_DestroyActor`)))

(fn `Rush`
  (returns (Location :type "Vector Structure"))
  (bind _returnvalue (* (`self.RushDistance`) 100.0))
  (bind (_returnvalue_x _returnvalue_y) (`KismetMathLibrary.BreakVector` (* (`KismetMathLibrary.GetForwardVector` (`KismetMathLibrary.FindLookAtRotation` (`self.K2_GetActorLocation`) (`self.K2_GetActorLocation` (`self.As BP Top Down Character`)))) (`KismetMathLibrary.MakeVector` _returnvalue _returnvalue))))
  (return (+ (`self.K2_GetActorLocation`) (`KismetMathLibrary.MakeVector` _returnvalue_x _returnvalue_y))))

(fn `UserConstructionScript`)