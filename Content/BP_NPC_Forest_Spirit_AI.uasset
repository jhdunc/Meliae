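; Forest spirit NPC character that follows the player and can trade places with them.
; It tracks the player with continuous AI MoveTo until GoToMouse pauses following and nudges it toward a given destination with movement input.
; A retriggerable five-second delay resumes following after the last GoToMouse call.
; While paused, SwapPlaces teleports the spirit to a passed destination and the player to the spirit's previous location.
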(event `self.ReceiveBeginPlay`
  (bind _asbp_top_down_character (cast `/Game/TopDown/Blueprints/BP_TopDownCharacter` (`GameplayStatics.GetPlayerCharacter` 0)))
  (set `self.As BP Top Down Character` _asbp_top_down_character)
  (`self.Go To Player`))

(event `Go To Mouse`
  (params (Destination :type "Vector Structure"))
  (set `self.Paused` true)
  (`Controller.StopMovement` (`AIBlueprintHelperLibrary.GetAIController` self))
  (`PawnMovementComponent.AddInputVector` (`self.CharacterMovement`) (`KismetMathLibrary.GetForwardVector` (`KismetMathLibrary.FindLookAtRotation` (`self.K2_GetActorLocation`) Destination)) false)
  (`KismetSystemLibrary.RetriggerableDelay` 5.0)
  (set `self.Paused` false)
  (`self.Go To Player`))

(event `Go To Player`
  (if (not (`self.Paused`))
    (`AITask_MoveTo.AIMoveTo` (`AIBlueprintHelperLibrary.GetAIController` self) (0.0 0.0 0.0) (`self.As BP Top Down Character`) -1.0 "Disable" "Enable" true false true "Enable")))

(event `Swap Places`
  (params (Destination :type "Vector Structure"))
  (if (`self.Paused`)
    (bind _output_get (set `self.TempLocation` (`self.K2_GetActorLocation`)))
    (`self.K2_SetActorLocation` Destination false true)
    (`self.K2_SetActorLocation` (`self.As BP Top Down Character`) _output_get false true)))

(fn `UserConstructionScript`)