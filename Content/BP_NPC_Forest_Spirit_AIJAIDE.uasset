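; Forest spirit companion NPC that frees itself shortly after spawn, follows the player and detours to drops when the player is below max health.
; Following re-issues AIMoveTo; failed moves at a distance start a looping timer that teleports it to the player's FriendTeleportSpot once OnFallingBlock is false.
; Drop trips pause following and show the WB_FriendAlert widget.
; GoToMouse and SwapPlaces are empty, with leftover move and swap logic disconnected.
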(event `Go To Mouse`
  (params (Destination :type "Vector Structure")))

(event `Freed`
  (`ActorComponent.K2_DestroyComponent` (`self.StaticMesh`))
  (set `self.IsFree?` true)
  (`self.Go To Player`))

(event `self.ReceiveBeginPlay`
  (bind _asbp_top_down_character (cast `/Game/TopDown/Blueprints/BP_TopDownCharacter` (`GameplayStatics.GetPlayerCharacter` 0)))
  (set `self.As BP Top Down Character` _asbp_top_down_character)
  (bind _foundwidgets (`WidgetBlueprintLibrary.GetAllWidgetsOfClass` "/Game/GameFilesMeliae/UI/WB_FriendAlert.WB_FriendAlert_C" false))
  (set `self.Widget` (`|GetArrayItem` _foundwidgets))
  (`KismetSystemLibrary.Delay` 2.5)
  (`self.Freed`))

(event `Go To Player`
  (if (`self.Paused`)
    (`KismetSystemLibrary.Delay` 0.2)
    (`self.Go To Player` :!label _label)
    (else
      (`AITask_MoveTo.AIMoveTo` (`AIBlueprintHelperLibrary.GetAIController` self) (0.0 0.0 0.0) (`self.As BP Top Down Character`) (`self.DistanceFromPlayer`) "Enable" "Enable" true false
        (:`OnRequestFailed`
          (if (>= (`KismetMathLibrary.Vector_Distance` (`self.K2_GetActorLocation` (`GameplayStatics.GetPlayerCharacter` 0)) (`self.K2_GetActorLocation`)) 70.0)
            (`KismetSystemLibrary.K2_SetTimer` null "TryTeleport" 0.33 true)
            (else
              (`self.Go To Player`))))
        (:`OnMoveFinished`
          (`KismetSystemLibrary.Delay` 0.0)
          (goto _label))))))

(event `Swap Places`
  (params (Destination :type "Vector Structure")))

(event `Go To Drop`
  (params (TargetLocation :type "Vector Structure"))
  (bind _as_bp_top_down_character (`self.As BP Top Down Character`))
  (if (`self.IsFree?`)
    (`KismetSystemLibrary.PrintString` "Ooh shiny")
    (if (== (`/Game/TopDown/Blueprints/BP_TopDownCharacter.CurrentHealth` _as_bp_top_down_character) (`/Game/TopDown/Blueprints/BP_TopDownCharacter.MaxHealth` _as_bp_top_down_character))
      (`KismetSystemLibrary.PrintString` "heal condition true")
      (else
        (`KismetSystemLibrary.PrintString` "heal condition false")
        (set `self.Paused` true)
        (`AITask_MoveTo.AIMoveTo` (`AIBlueprintHelperLibrary.GetAIController` self) TargetLocation null -1.0 "Enable" "Enable" true true true
          (:`then`
            (`Widget.SetVisibility` (`self.Widget`) "Visible"))
          (:`OnRequestFailed`
            (`KismetSystemLibrary.PrintString` "Req Failed")
            (`KismetSystemLibrary.Delay` 0.5 :!label _label_2)
            (bind _output_get (set `self.Paused` false))
            (`KismetSystemLibrary.PrintString` (`KismetStringLibrary.Conv_BoolToString` _output_get))
            (`Widget.SetVisibility` (`self.Widget`) "Hidden"))
          (:`OnMoveFinished`
            (`KismetSystemLibrary.PrintString` "Move Ended")
            (goto _label_2)))))))

(fn `RunToEnemy`
  (params (`Target Location` :type "Vector Structure"))
  (`self.Go To Drop` `Target Location`))

(fn `TryTeleport`
  (if (not (`/Game/TopDown/Blueprints/BP_TopDownCharacter.OnFallingBlock` (`self.As BP Top Down Character`)))
    (`self.K2_SetActorLocation` (`SceneComponent.K2_GetComponentLocation` (`/Game/TopDown/Blueprints/BP_TopDownCharacter.FriendTeleportSpot` (`self.As BP Top Down Character`))))
    (`self.Go To Player`)
    (`KismetSystemLibrary.K2_ClearTimer` null "TryTeleport")))

(fn `UserConstructionScript`)