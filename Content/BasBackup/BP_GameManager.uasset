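; Game manager Blueprint that tracks enemy counts and switches background music state as enemies appear and are cleared.
; SpawnUpdate grows the room maximum, refills the current count and sets second-stage music, while Tick computes the remaining ratio.
; A separate total-enemy counter restores first-stage music at zero.
; It also caches the forest spirit NPC reference and offers a chance-based health pickup spawn at a triggering actor's location.
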(event `self.ReceiveBeginPlay`
  (bind _returnvalue (`GameplayStatics.GetActorOfClass` "/Game/BP_NPC_Forest_Spirit_AI.BP_NPC_Forest_Spirit_AI_C"))
  (set `self.FriendReference` _returnvalue)
  (bind _output_get (set `self.RoomEnemyMax` 0))
  (set `self.RoomEnemyCurrent` _output_get))

(event `self.ReceiveTick`
  (params (DeltaSeconds :type "Float (single-precision)"))
  (set `self.RoomEnemyPercent` (/ (`KismetMathLibrary.Conv_IntToDouble` (`self.RoomEnemyCurrent`)) (`KismetMathLibrary.Conv_IntToDouble` (`self.RoomEnemyMax`))))
  (if (== (`self.RoomEnemyCurrent`) 0)
    (set `self.RoomEnemyMax` 0)))

(fn `SpawnPickup`
  (params (`Triggering Actor` :type "Actor Object Reference") (SpawnChance :type Integer))
  (if (<= (`KismetMathLibrary.RandomInteger` 100) SpawnChance)
    (`|SpawnActorFromClass` "/Game/TopDown/Blueprints/BP_HealthPickup.BP_HealthPickup_C" (`KismetMathLibrary.MakeTransform` (`KismetMathLibrary.MakeVector` (.x (`self.K2_GetActorLocation` `Triggering Actor`)) (.y (`self.K2_GetActorLocation` `Triggering Actor`)) (.z (`self.K2_GetActorLocation` `Triggering Actor`)))) "AlwaysSpawn" "MultiplyWithRoot" null null)
    (return)))

(fn `SpawnUpdate`
  (params (Health :type Integer))
  (bind _output_get (set `self.RoomEnemyMax` (+ Health (`self.RoomEnemyMax`))))
  (set `self.RoomEnemyCurrent` _output_get)
  (`AkGameplayStatics.SetState` "/Game/WwiseAudio/States/Default_Work_Unit/BackgroundMusicStateGroup/BackgroundMusicStateGroup-SecondStage.BackgroundMusicStateGroup-SecondStage"))

(fn `SubtractEnemyCurrent`
  (set `self.RoomEnemyCurrent` (- (`self.RoomEnemyCurrent`) 1)))

(fn `UpdateTotalEnemies`
  (params (Spawn :type Boolean))
  (bind _totalenemies (`self.TotalEnemies`))
  (if Spawn
    (set `self.TotalEnemies` (+ _totalenemies 1))
    (else
      (set `self.TotalEnemies` (- _totalenemies 1))))
  (bind _output_get (set `self.NoEnemiesLeft` (== _totalenemies 0)))
  (if _output_get
    (`AkGameplayStatics.SetState` "/Game/WwiseAudio/States/Default_Work_Unit/BackgroundMusicStateGroup/BackgroundMusicStateGroup-FirstStage.BackgroundMusicStateGroup-FirstStage")))

(fn `UserConstructionScript`)