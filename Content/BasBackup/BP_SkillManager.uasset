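; Skill manager actor that handles the player character's active skills in a top-down game.
; E cycles four slots, and IA_Shoot fires either a delayed, montage-backed projectile or a cooldown-gated fan of thorn projectiles; other slots do nothing.
; A shield function spawns an attached, movement-slowing shield if unlocked, but its input event is empty.
; Tick runs the shield cooldown reset, and several older shield, bubble and thorn chains remain disconnected.
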(event `Key|E`
  (params (Key :type "Key Structure"))
  (:`Pressed`
    ;[0.8549 0.2902 0.05098] Skill Up/Down
    (if (!= (`self.ActiveSkillLMB`) 4)
      (bind _output_get (set `self.ActiveSkillLMB` (+ (`self.ActiveSkillLMB`) 1)))
      (`KismetSystemLibrary.PrintString` (`KismetStringLibrary.Conv_IntToString` (`KismetMathLibrary.Clamp` _output_get 1 4)))
      (else
        (bind _output_get_2 (set `self.ActiveSkillLMB` 1))
        (`KismetSystemLibrary.PrintString` (`KismetStringLibrary.Conv_IntToString` (`KismetMathLibrary.Clamp` _output_get_2 1 4)))))))

(event `Key|Q`
  (params (Key :type "Key Structure")))

(event `Skill Bullet Fire`
  ;[1 1 1 0.1] Base Skill Behavior
  ;;[0.8549 0.2902 0.05098] SKILL : Single Projectile
  (`/Engine/EditorBlueprintResources/StandardMacros.Gate` true :!label _label))

(event `Key|LeftMouseButton`
  (params (Key :type "Key Structure"))
  ;[1 1 1 0.1] Base Skill Behavior
  ;;[0.8549 0.2902 0.05098] SKILL : Single Projectile
  (:`Pressed`
    (goto _label :!via `Open`))
  (:`Released`
    (goto _label :!via `Close`)))

(event `EnhancedInput|/Game/TopDown/Input/Actions/Keyboard/IA_Shoot`
  (params (ActionValue :type Boolean) (ElapsedSeconds :type "Float (double-precision)") (TriggeredSeconds :type "Float (double-precision)") (InputAction :type "InputAction Object Reference" :default "/Game/TopDown/Input/Actions/Keyboard/IA_Shoot.IA_Shoot"))
  (bind _playerref (`self.PlayerRef`))
  ;[1 1 1 0.1] Base Skill Behavior
  ;;[0.8549 0.2902 0.05098] SKILL : Single Projectile
  (:`Triggered`
    (set `/Game/TopDown/Blueprints/BP_TopDownCharacter.TriggerAnimation` true (`self.PlayerRef`))
    (switch `int` (`self.ActiveSkillLMB`)
      (:`1`
        (`KismetSystemLibrary.Delay` (`self.FireRate`))
        (`Character.PlayAnimMontage` _playerref "/Game/GameFilesMeliae/Characters/Animations/AM_Shooting.AM_Shooting" 1.0 "None")
        (set `/Game/TopDown/Blueprints/BP_TopDownCharacter.TriggerAnimation` false _playerref)
        (bind _returnvalue (`|SpawnActorFromClass` "/Game/TopDown/Blueprints/BP_Projectile.BP_Projectile_C" (`SceneComponent.K2_GetComponentToWorld` (`/Game/TopDown/Blueprints/BP_TopDownCharacter.BulletSpawn` (`self.PlayerRef`))) "Undefined" "MultiplyWithRoot" null (`self.Damage`) 1000.0 null))
        (if (`KismetSystemLibrary.IsValid` _returnvalue)
          (`self.SetLifeSpan` _returnvalue (`self.BulletLifespan`))
          ;;;[0.1294 0.02353 0.451] Post evet
          (`AkGameplayStatics.PostEvent` "/Game/WwiseAudio/Events/Default_Work_Unit/Player/Shoot/PlayerShoot.PlayerShoot")))
      (:`2`
        (`self.ThornSkill`)))))

(event `Key|RightMouseButton`
  (params (Key :type "Key Structure"))
  ;[1 1 1 0.1] Base Skill Behavior
  ;;[0.8549 0.2902 0.05098 0.1] SKILL : SHIELD DEFUNCT
)

(event `self.ReceiveBeginPlay`
  (bind _asbp_top_down_character (cast `/Game/TopDown/Blueprints/BP_TopDownCharacter` (`GameplayStatics.GetPlayerCharacter` 0)))
  (set `self.PlayerRef` _asbp_top_down_character)
  (`self.EnableInput` (`GameplayStatics.GetPlayerController` 0)))

(event `self.ReceiveTick`
  (params (DeltaSeconds :type "Float (single-precision)"))
  (`self.ShieldCD_Delay` (`self.ShieldCooldownAmt`)))

(event `EnhancedInput|/Game/TopDown/Input/Actions/Keyboard/IA_Shield`
  (params (ActionValue :type Boolean) (ElapsedSeconds :type "Float (double-precision)") (TriggeredSeconds :type "Float (double-precision)") (InputAction :type "InputAction Object Reference" :default "/Game/TopDown/Input/Actions/Keyboard/IA_Shield.IA_Shield"))
  ;[0.8549 0.2902 0.05098 0.1] SKILL : Shield
)

(fn `ShieldSkill`
  (params (ShieldLifespan :type "Float (double-precision)"))
  (bind _playerref (`self.PlayerRef`))
  ;[0.8549 0.2902 0.05098 0.1] SKILL : Shield
  (if (`self.ShieldCD`)
    _
    (elif (`BlueprintSetLibrary.Set_Contains` (`/Game/TopDown/Blueprints/BP_TopDownCharacter.SkillList` (`self.PlayerRef`)) 2)
      (set `self.ShieldCD` true)
      (if (not (`KismetSystemLibrary.IsValid` (`self.Shield Var`)))
        ;;[0.8549 0.2902 0.05098 0.102] Spawn Shield Actor
        (bind _returnvalue (`|SpawnActorFromClass` "/Game/TopDown/Blueprints/Greybox/BP_Shield.BP_Shield_C" (`SceneComponent.K2_GetComponentToWorld` (`/Game/TopDown/Blueprints/BP_TopDownCharacter.BulletSpawn` (`self.PlayerRef`))) "AdjustIfPossibleButAlwaysSpawn" "MultiplyWithRoot" null null))
        (bind _output_get (set `self.Shield Var` _returnvalue))
        (`self.SetLifeSpan` _output_get ShieldLifespan)
        (`self.K2_AttachToActor` (`self.PlayerRef`) "None" "SnapToTarget" "SnapToTarget" "KeepRelative")
        (set `/Game/TopDown/Blueprints/BP_TopDownCharacter.SlowEffects` (+ (`/Game/TopDown/Blueprints/BP_TopDownCharacter.SlowEffects` _playerref) 1) _playerref)
        (`/Game/TopDown/Blueprints/BP_TopDownCharacter.Set Movement` _playerref 200.0 (`/Game/TopDown/Blueprints/BP_TopDownCharacter.CharRotSpeedDefault` _playerref)))
      (else
        (`KismetSystemLibrary.PrintString` "Skill is Not Unlocked")))))

(fn `UnlockShield`
  (bind _skilllist (`/Game/TopDown/Blueprints/BP_TopDownCharacter.SkillList` (`self.PlayerRef`)))
  (if (not (`BlueprintSetLibrary.Set_Contains` _skilllist 2))
    (`BlueprintSetLibrary.Set_Add` _skilllist 2)))

(fn `UserConstructionScript`)