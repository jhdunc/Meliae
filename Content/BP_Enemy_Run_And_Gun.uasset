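; Top-down run-and-gun enemy that charges the player, shoots, then retreats.
; A recursive AI MoveTo loop runs to the player's position, fires a projectile, then moves to RunAwayPoint, while a delay loop keeps it facing the player.
; It deals contact damage, may spawn pickups when hit, and updates GameManager room totals and the player's enemy counter.
; Older proximity, movement and damage logic is disconnected, and the health bar refreshes only at BeginPlay.
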(event `self.ReceiveBeginPlay`
  (bind _as_bp_top_down_character (`self.As BP Top Down Character`))
  (bind _gamemanager (`self.GameManager`))
  (bind _returnvalue (`GameplayStatics.GetActorOfClass` "/Game/TopDown/Blueprints/BP_GameManager.BP_GameManager_C"))
  (set `self.GameManager` _returnvalue)
  (bind _asbp_top_down_character (cast `/Game/TopDown/Blueprints/BP_TopDownCharacter` (`GameplayStatics.GetPlayerCharacter` 0)))
  (set `self.As BP Top Down Character` _asbp_top_down_character)
  (`self.Rotate`)
  (set `/Game/TopDown/Blueprints/BP_TopDownCharacter.EnemyCounter` (+ (`/Game/TopDown/Blueprints/BP_TopDownCharacter.EnemyCounter` _as_bp_top_down_character) 1) _as_bp_top_down_character)
  (set `self.Health` (`self.MaxHealth`))
  (`self.UpdateHealthbar`)
  (bind _output_get (set `/Game/TopDown/Blueprints/BP_GameManager.RoomEnemyMax` (+ (`/Game/TopDown/Blueprints/BP_GameManager.RoomEnemyMax` _gamemanager) (`self.Health`)) _gamemanager))
  (set `/Game/TopDown/Blueprints/BP_GameManager.RoomEnemyCurrent` _output_get _gamemanager)
  (`self.Movement`))

(event `Rotate`
  (`self.K2_SetActorRotation` (`KismetMathLibrary.MakeRotator` 0.0 0.0 (.yaw (`KismetMathLibrary.RInterpTo` (`self.K2_GetActorRotation`) (`KismetMathLibrary.FindLookAtRotation` (`self.K2_GetActorLocation`) (`self.K2_GetActorLocation` (`self.As BP Top Down Character`))) (`GameplayStatics.GetWorldDeltaSeconds`) 25.0))))
  (`KismetSystemLibrary.Delay` 0.01)
  (`self.Rotate`))

(event `self.ReceiveAnyDamage`
  (params (Damage :type "Float (single-precision)") (DamageType :type "DamageType Object Reference") (InstigatedBy :type "Controller Object Reference") (DamageCauser :type "Actor Object Reference"))
  (bind _gamemanager (`self.GameManager`))
  ;[0.8549 0.2902 0.05098] On Damage Update Health
  (`/Game/TopDown/Blueprints/BP_GameManager.SpawnPickup` (`self.GameManager`) self 4)
  (set `self.Health` (- (`self.Health`) (`KismetMathLibrary.Round` Damage)))
  (set `/Game/TopDown/Blueprints/BP_GameManager.RoomEnemyCurrent` (- (`/Game/TopDown/Blueprints/BP_GameManager.RoomEnemyCurrent` _gamemanager) 1) _gamemanager)
  (if (<= (`self.Health`) 0)
    (`self.K2_DestroyActor`)))

(event `self.ReceiveTick`
  (params (DeltaSeconds :type "Float (single-precision)"))
  ;[0 0.0549 0.1686] Old Movement
)

(event `self.HitBox.OnComponentBeginOverlap`
  (params (OverlappedComponent :type "PrimitiveComponent Object Reference") (OtherActor :type "Actor Object Reference") (OtherComp :type "PrimitiveComponent Object Reference") (OtherBodyIndex :type Integer) (bFromSweep :type Boolean) (SweepResult :type "HitResult Structure (by ref)"))
  ;[0 0.0549 0.1686] Contact Damage
  (bind _asbp_top_down_character (cast `/Game/TopDown/Blueprints/BP_TopDownCharacter` OtherActor))
  (`GameplayStatics.ApplyDamage` _asbp_top_down_character 1.0))

(event `Movement`
  (bind (_returnvalue_x _returnvalue_y _returnvalue_z) (`KismetMathLibrary.BreakVector` (`self.K2_GetActorLocation`)))
  (bind (_returnvalue_x_2 _returnvalue_y_2) (`KismetMathLibrary.BreakVector` (`self.K2_GetActorLocation` (`GameplayStatics.GetPlayerCharacter` 0))))
  (`KismetSystemLibrary.Delay` 0.5)
  (`AITask_MoveTo.AIMoveTo` (`AIBlueprintHelperLibrary.GetAIController` self) (`KismetMathLibrary.MakeVector` _returnvalue_x_2 _returnvalue_y_2 _returnvalue_z) null 450.0 "Enable" "Enable"
    (:`OnRequestFailed`
      (`self.Movement`))
    (:`OnMoveFinished`
      (`KismetSystemLibrary.Delay` (`KismetMathLibrary.RandomFloatInRange` 0.15 0.25))
      (`self.FireBullet`)
      (`AITask_MoveTo.AIMoveTo` (`AIBlueprintHelperLibrary.GetAIController` self) (`SceneComponent.K2_GetComponentLocation` (`self.RunAwayPoint`)) null -1.0 "Default" "Enable"
        (:`OnRequestFailed`
          _)
        (:`OnMoveFinished`
          _))
      (`self.Movement`))))

(event `self.ReceiveDestroyed`
  (bind _as_bp_top_down_character (`self.As BP Top Down Character`))
  (set `/Game/TopDown/Blueprints/BP_TopDownCharacter.EnemyCounter` (- (`/Game/TopDown/Blueprints/BP_TopDownCharacter.EnemyCounter` _as_bp_top_down_character) 1) _as_bp_top_down_character))

(fn `FireBullet`
  ;[0 0.0549 0.1686] Fire Bullet
  (`|SpawnActorFromClass` "/Game/BP_Enemy_Run_And_Gun_Projectile.BP_Enemy_Run_And_Gun_Projectile_C" (`KismetMathLibrary.MakeTransform` (`SceneComponent.K2_GetComponentLocation` (`self.BulletSpawnPoint`)) (`self.K2_GetActorRotation`) (0.4 0.4 0.4)) "AdjustIfPossibleButAlwaysSpawn" "MultiplyWithRoot" null null))

(fn `Jiggle`
  (bind _returnvalue (`KismetMathLibrary.MakeVector` (* (.x (`KismetMathLibrary.GetRightVector` (`self.K2_GetActorRotation`))) 1000.0) (* (.y (`KismetMathLibrary.GetRightVector` (`self.K2_GetActorRotation`))) 1000.0)))
  (`KismetSystemLibrary.PrintString` (`KismetStringLibrary.Conv_VectorToString` _returnvalue))
  (`PawnMovementComponent.AddInputVector` (`self.FloatingPawnMovement`) _returnvalue false))

(fn `UpdateHealthbar`
  (bind _aswb_enemy_health (cast `/Game/GameFilesMeliae/UI/WB_EnemyHealth` (`WidgetComponent.GetUserWidgetObject` (`self.HealthBarWidget`))))
  (set `/Game/GameFilesMeliae/UI/WB_EnemyHealth.Health` (/ (`KismetMathLibrary.Conv_IntToDouble` (`self.Health`)) (`KismetMathLibrary.Conv_IntToDouble` (`self.MaxHealth`))) _aswb_enemy_health)
  (return))

(fn `UserConstructionScript`)