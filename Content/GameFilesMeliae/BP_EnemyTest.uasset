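; BP_EnemyTest is a test enemy that stays dormant and ignores hits until a BP_TopDownCharacter overlaps its Sphere trigger.
; Activation starts a looping timer calling FireBullets, which spawns BP_Run_And_Gun_Projectile in an evenly spaced ring from the Cube.
; The ring's bullet count alternates between full and half on successive volleys.
; Once active, BP_Projectile overlaps on the Cube subtract rounded damage from Health, destroying the enemy at zero or below.
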(event `self.ReceiveBeginPlay`)

(event `self.Cube.OnComponentBeginOverlap`
  (params (OverlappedComponent :type "PrimitiveComponent Object Reference") (OtherActor :type "Actor Object Reference") (OtherComp :type "PrimitiveComponent Object Reference") (OtherBodyIndex :type Integer) (bFromSweep :type Boolean) (SweepResult :type "HitResult Structure (by ref)"))
  (if (`self.Active`)
    (bind _asbp_projectile (cast `/Game/TopDown/Blueprints/BP_Projectile` OtherActor))
    (bind _output_get (set `self.Health` (- (`self.Health`) (`KismetMathLibrary.Round` (`/Game/TopDown/Blueprints/BP_Projectile.Damage` _asbp_projectile)))))
    (`self.K2_DestroyActor` _asbp_projectile)
    (if (<= _output_get 0)
      (`self.K2_DestroyActor`))))

(event `self.Sphere.OnComponentBeginOverlap`
  (params (OverlappedComponent :type "PrimitiveComponent Object Reference") (OtherActor :type "Actor Object Reference") (OtherComp :type "PrimitiveComponent Object Reference") (OtherBodyIndex :type Integer) (bFromSweep :type Boolean) (SweepResult :type "HitResult Structure (by ref)"))
  (if (not (`self.Active`))
    (cast `/Game/TopDown/Blueprints/BP_TopDownCharacter` OtherActor)
    (`|ExecutionSequence`
      (:`then_0`
        (set `self.Active` true)
        (`KismetSystemLibrary.PrintString` "Activate"))
      (:`then_1`
        (set `self.BulletsTemp` (/ (`self.BulletsAmount`) 2))
        (`KismetSystemLibrary.K2_SetTimer` null "FireBullets" 4.0 true 1.0)))))

(fn `FireBullets`
  (locals (Tag :type "Array of Name"))
  (bind _bulletsamount (`self.BulletsAmount`))
  (for _index (range _bulletsamount)
    (`|SpawnActorFromClass` "/Game/BP_Run_And_Gun_Projectile.BP_Run_And_Gun_Projectile_C" (`KismetMathLibrary.MakeTransform` (`SceneComponent.K2_GetComponentLocation` (`self.Cube`)) (`KismetMathLibrary.MakeRotator` 0.0 0.0 (`KismetMathLibrary.Conv_IntToDouble` (* _index (/ 360 _bulletsamount))))) "Undefined" "MultiplyWithRoot" null null))
  (if (== (`self.BulletsAmount`) (`self.BulletsTemp`))
    (set `self.BulletsAmount` (* (`self.BulletsAmount`) 2))
    (else
      (set `self.BulletsAmount` (`self.BulletsTemp`)))))

(fn `UserConstructionScript`)