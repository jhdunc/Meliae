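; BP_DamageFlash is a component that briefly flashes its owner's emissive material when the owner takes damage.
; On BeginPlay it binds to OnTakeAnyDamage, creates a dynamic material on slot 0 of the owner's first static mesh, and caches the emissive color and multiplier.
; The damage handler applies the flash color and intensity, waits for the flash duration, then restores the cached values.
; It also prints the owner's name on BeginPlay.
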(event `self.ReceiveBeginPlay`
  (bind _returnvalue (`self.GetOwner`))
  (bind _flashmat (`self.FlashMat`))
  (bind _returnvalue_2 (`Actor.GetComponentByClass` (`self.Owner`) "/Script/Engine.StaticMeshComponent"))
  (set `self.Owner` _returnvalue)
  (add `Actor.OnTakeAnyDamage` _returnvalue (`|CreateDelegate` :!event `DamageFlash`))
  ;[0 0.9257 1] Setup dynamic material instance from actor
  (`KismetSystemLibrary.PrintString` (`KismetSystemLibrary.GetDisplayName` _returnvalue))
  (`/Engine/EditorBlueprintResources/StandardMacros.IsValid` _returnvalue_2
    (:`Is Valid`
      (bind _returnvalue_3 (`PrimitiveComponent.CreateDynamicMaterialInstance` _returnvalue_2 0 null "None"))
      (set `self.FlashMat` _returnvalue_3)
      ;[0 1 0.9263] Save initial values
      (bind _returnvalue_4 (`MaterialInstanceDynamic.K2_GetVectorParameterValue` _flashmat "EmissiveColor"))
      (set `self.InitEmissiveColor` _returnvalue_4)
      (bind _returnvalue_5 (`MaterialInstanceDynamic.K2_GetScalarParameterValue` _flashmat "EmissiveMultiplier"))
      (set `self.InitEmissiveMultiplier` _returnvalue_5))))

(event `DamageFlash`
  (params (DamagedActor :type "Actor Object Reference") (Damage :type "Float (single-precision)") (DamageType :type "DamageType Object Reference") (InstigatedBy :type "Controller Object Reference") (DamageCauser :type "Actor Object Reference"))
  (bind _flashmat (`self.FlashMat`))
  (bind _flashmat_2 (`self.FlashMat`))
  ;[0 0.9618 1] edit values
  (`MaterialInstanceDynamic.SetVectorParameterValue` _flashmat_2 "EmissiveColor" (`self.FlashColor`))
  (`MaterialInstanceDynamic.SetScalarParameterValue` _flashmat_2 "EmissiveMultiplier" (`self.FlashIntensity`))
  (`KismetSystemLibrary.Delay` (`self.FlashDuration`))
  ;[0 0.9413 1] return to original values
  (`MaterialInstanceDynamic.SetVectorParameterValue` _flashmat "EmissiveColor" (`self.InitEmissiveColor`))
  (`MaterialInstanceDynamic.SetScalarParameterValue` _flashmat "EmissiveMultiplier" (`self.InitEmissiveMultiplier`)))