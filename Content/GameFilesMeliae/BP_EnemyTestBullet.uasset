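; BP_EnemyTestBullet is a test enemy projectile that damages the top-down player character.
; A custom event receives the other actor, subtracts Damage from a BP_TopDownCharacter's CurrentHealth, prints debug text and destroys the bullet.
; For other actors it destroys itself unless they are tagged Bullet or Enemy.
; An older hard-coded damage branch remains in the graph but never runs.
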(event `CustomEvent`
  (params (OtherActor :type "Actor Object Reference"))
  (bind _asbp_top_down_character (cast `/Game/TopDown/Blueprints/BP_TopDownCharacter` OtherActor)
    (:`then`
      (`KismetSystemLibrary.PrintString` "Hit")
      (bind _output_get (set `/Game/TopDown/Blueprints/BP_TopDownCharacter.CurrentHealth` (- (`/Game/TopDown/Blueprints/BP_TopDownCharacter.CurrentHealth` _asbp_top_down_character) (`KismetMathLibrary.Conv_IntToDouble` (`self.Damage`))) _asbp_top_down_character))
      (`KismetSystemLibrary.PrintString` (`KismetStringLibrary.Conv_DoubleToString` _output_get))
      (`self.K2_DestroyActor`))
    (:`CastFailed`
      (if (not (or (`self.ActorHasTag` OtherActor "Bullet") (`self.ActorHasTag` OtherActor "Enemy")))
        (`self.K2_DestroyActor`)))))

(fn `UserConstructionScript`)