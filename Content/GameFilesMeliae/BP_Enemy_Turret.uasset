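; Stationary-style enemy turret that wakes when the player character enters its detection sphere, then fires radial bullet bursts.
; On activation a looping timer calls FireBullets, which spawns evenly spaced projectiles in a ring, alternating between full and half bullet count.
; Its hitbox damages the player on overlap.
; Each hit taken requests a pickup spawn from BP_GameManager and reduces health, destroying the turret at zero.
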(event `self.ReceiveBeginPlay`
  (bind _returnvalue (`GameplayStatics.GetActorOfClass` "/Game/TopDown/Blueprints/BP_GameManager.BP_GameManager_C"))
  (set `self.GameManager` _returnvalue))

(event `self.ReceiveAnyDamage`
  (params (Damage :type "Float (single-precision)") (DamageType :type "DamageType Object Reference") (InstigatedBy :type "Controller Object Reference") (DamageCauser :type "Actor Object Reference"))
  (`/Game/TopDown/Blueprints/BP_GameManager.SpawnPickup` (`self.GameManager`) self 4)
  (bind _output_get (set `self.Health` (- (`self.Health`) (`KismetMathLibrary.Round` Damage))))
  (if (<= _output_get 0)
    (`self.K2_DestroyActor`)))

(event `self.Sphere.OnComponentBeginOverlap`
  (params (OverlappedComponent :type "PrimitiveComponent Object Reference") (OtherActor :type "Actor Object Reference") (OtherComp :type "PrimitiveComponent Object Reference") (OtherBodyIndex :type Integer) (bFromSweep :type Boolean) (SweepResult :type "HitResult Structure (by ref)"))
  (if (not (`self.Active`))
    (cast `/Game/TopDown/Blueprints/BP_TopDownCharacter` OtherActor)
    (`|ExecutionSequence`
      (:`then_0`
        (set `self.Active` true))
      (:`then_1`
        (set `self.BulletsTemp` (/ (`self.BulletsAmount`) 2))
        (`KismetSystemLibrary.K2_SetTimer` null "FireBullets" 4.0 true 1.0)))))

(event `self.HitBox.OnComponentBeginOverlap`
  (params (OverlappedComponent :type "PrimitiveComponent Object Reference") (OtherActor :type "Actor Object Reference") (OtherComp :type "PrimitiveComponent Object Reference") (OtherBodyIndex :type Integer) (bFromSweep :type Boolean) (SweepResult :type "HitResult Structure (by ref)"))
  (bind _asbp_top_down_character (cast `/Game/TopDown/Blueprints/BP_TopDownCharacter` OtherActor))
  (`GameplayStatics.ApplyDamage` _asbp_top_down_character 1.0))

(fn `FireBullets`
  (locals (Tag :type "Array of Name"))
  (bind _bulletsamount (`self.BulletsAmount`))
  (for _index (range _bulletsamount)
    (`|SpawnActorFromClass` "/Game/Projectiles/BP_Enemy_Run_And_Gun_Projectile.BP_Enemy_Run_And_Gun_Projectile_C" (`KismetMathLibrary.MakeTransform` (`SceneComponent.K2_GetComponentLocation` (`self.Cube`)) (`KismetMathLibrary.MakeRotator` 0.0 0.0 (`KismetMathLibrary.Conv_IntToDouble` (* _index (/ 360 _bulletsamount))))) "Undefined" "MultiplyWithRoot" null null))
  (if (== (`self.BulletsAmount`) (`self.BulletsTemp`))
    (set `self.BulletsAmount` (* (`self.BulletsAmount`) 2))
    (else
      (set `self.BulletsAmount` (`self.BulletsTemp`)))))

(fn `UserConstructionScript`)