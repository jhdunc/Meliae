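; Projectile for a Run and Gun attack that damages the top-down player character on contact.
; On overlap it casts to BP_TopDownCharacter, applies its Damage, prints the character's current health and destroys itself.
; Any other overlapped actor also destroys it, unless tagged Bullet or Enemy, so it passes through those.
; An older direct health subtraction remains in the graph but is disconnected.
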(event `self.ReceiveActorBeginOverlap`
  (params (OtherActor :type "Actor Object Reference"))
  ;[0 0.0549 0.1686] ProjectileBehavior
  (bind _asbp_top_down_character (cast `/Game/TopDown/Blueprints/BP_TopDownCharacter` OtherActor)
    (:`then`
      ;;[0.8549 0.2902 0.05098] Cause Damage
      (`GameplayStatics.ApplyDamage` _asbp_top_down_character (`self.Damage`))
      (`KismetSystemLibrary.PrintString` (`KismetStringLibrary.Conv_DoubleToString` (`/Game/TopDown/Blueprints/BP_TopDownCharacter.CurrentHealth` _asbp_top_down_character)))
      (`self.K2_DestroyActor`))
    (:`CastFailed`
      (if (not (or (`self.ActorHasTag` OtherActor "Bullet") (`self.ActorHasTag` OtherActor "Enemy")))
        (`self.K2_DestroyActor`)))))

(fn `UserConstructionScript`)