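; Second-stage miniboss booster projectile that damages the player and splits into a ring of stage 3 projectiles.
; After a short delay from BeginPlay, it spawns eight evenly yawed BP_Miniboss_BoosterStage3_Projectile actors and destroys itself.
; HitBox overlap damages a vulnerable player and increments the GameInstance boss-hit stat, printing it.
; It is destroyed on any player contact or other overlap, except actors tagged Bullet, Enemy or Friend.
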(event `self.HitBox.OnComponentBeginOverlap`
  (params (OverlappedComponent :type "PrimitiveComponent Object Reference") (OtherActor :type "Actor Object Reference") (OtherComp :type "PrimitiveComponent Object Reference") (OtherBodyIndex :type Integer) (bFromSweep :type Boolean) (SweepResult :type "HitResult Structure (by ref)"))
  ;[0 0.0549 0.1686] ProjectileBehavior
  (bind _asbp_top_down_character (cast `/Game/TopDown/Blueprints/BP_TopDownCharacter` OtherActor)
    (:`then`
      ;;[0.8549 0.2902 0.05098] Cause Damage
      (if (not (`/Game/TopDown/Blueprints/BP_TopDownCharacter.Invulnerable` _asbp_top_down_character))
        (`GameplayStatics.ApplyDamage` _asbp_top_down_character (`self.Damage`))
        (`self.DamageBoop`
          (:`  `
            _)
          (:`then`
            _)))
      (`self.K2_DestroyActor`))
    (:`CastFailed`
      (if (not (or (`self.ActorHasTag` OtherActor "Bullet") (`self.ActorHasTag` OtherActor "Enemy") (`self.ActorHasTag` OtherActor "Friend")))
        (`self.K2_DestroyActor`)))))

(event `self.ReceiveBeginPlay`
  (`KismetSystemLibrary.Delay` 0.66)
  (for _index (range 8)
    (`|SpawnActorFromClass` "/Game/BP_Miniboss_BoosterStage3_Projectile.BP_Miniboss_BoosterStage3_Projectile_C" (`KismetMathLibrary.MakeTransform` (`self.K2_GetActorLocation`) (`KismetMathLibrary.MakeRotator` 0.0 0.0 (`KismetMathLibrary.Conv_IntToDouble` (* _index (/ 360 8))))) "Undefined" "MultiplyWithRoot" null null))
  (`self.K2_DestroyActor`))

(fn `UserConstructionScript`)