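; Falling-projectile actor for the miniboss's flying attack, judging by its name and the indicator it targets.
; Its HitBox overlap destroys it only on touching a BP_Enemy_Miniboss_FlyingAttack_Indicator, ignoring all other actors.
; Player damage, tag-filtered destruction and the DamageBoop hit counter (TimesHitByBoss in the stats game instance) remain only in disconnected code, so this projectile deals no damage itself.
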(event `self.HitBox.OnComponentBeginOverlap`
  (params (OverlappedComponent :type "PrimitiveComponent Object Reference") (OtherActor :type "Actor Object Reference") (OtherComp :type "PrimitiveComponent Object Reference") (OtherBodyIndex :type Integer) (bFromSweep :type Boolean) (SweepResult :type "HitResult Structure (by ref)"))
  ;[0 0.0549 0.1686] ProjectileBehavior
  (cast `/Game/Projectiles/BP_Enemy_Miniboss_FlyingAttack_Indicator` OtherActor)
  (`self.K2_DestroyActor`))

(fn `UserConstructionScript`)