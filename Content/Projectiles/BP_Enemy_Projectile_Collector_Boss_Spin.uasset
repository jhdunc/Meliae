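; BP_Enemy_Projectile_Collector_Boss_Spin is an enemy projectile, named for the Collector boss's spin attack, that damages the player on overlap.
; A HitBox overlap with BP_TopDownCharacter applies damage unless the character is invulnerable, then destroys the projectile either way.
; Each damaging hit calls DamageBoop, which increments TimesHitByBoss in the stats GameInstance.
; Other overlaps destroy it, except actors tagged Bullet, Enemy or Friend.
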(event `self.HitBox.OnComponentBeginOverlap`
  (params (OverlappedComponent :type "PrimitiveComponent Object Reference") (OtherActor :type "Actor Object Reference") (OtherComp :type "PrimitiveComponent Object Reference") (OtherBodyIndex :type Integer) (bFromSweep :type Boolean) (SweepResult :type "HitResult Structure (by ref)"))
  ;[0 0.0549 0.1686] ProjectileBehavior
  (bind _asbp_top_down_character (cast `/Game/TopDown/Blueprints/BP_TopDownCharacter` OtherActor)
    (:`then`
      ;;[0.8549 0.2902 0.05098] Cause Damage
      (if (not (`/Game/TopDown/Blueprints/BP_TopDownCharacter.Invulnerable` _asbp_top_down_character))
        (`GameplayStatics.ApplyDamage` _asbp_top_down_character (`self.Damage`))
        (`self.DamageBoop`
          (:`  `
            _)))
      (`self.K2_DestroyActor`))
    (:`CastFailed`
      (if (not (or (`self.ActorHasTag` OtherActor "Bullet") (`self.ActorHasTag` OtherActor "Enemy") (`self.ActorHasTag` OtherActor "Friend")))
        (`self.K2_DestroyActor`)))))

(fn `UserConstructionScript`)