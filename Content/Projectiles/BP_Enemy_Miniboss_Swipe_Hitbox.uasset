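; Short-lived melee swipe hitbox for an enemy miniboss that damages the player on contact.
; On BeginPlay a Timeline slides the Cube sideways along local Y, lerping from its current position each update, then the actor destroys itself after a brief delay.
; Cube overlaps with BP_TopDownCharacter apply damage unless that character is flagged Invulnerable.
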(event `self.ReceiveBeginPlay`
  (bind (_relativelocation_x _relativelocation_y) (`KismetMathLibrary.BreakVector` (`SceneComponent.RelativeLocation` (`self.Cube`))))
  (bind (_direction _newtrack_0) (`Timeline|Timeline` :!via `PlayFromStart`)
    (:`Update`
      (`SceneComponent.K2_SetRelativeLocation` (`self.Cube`) (`KismetMathLibrary.MakeVector` 0.0 (`KismetMathLibrary.Lerp` _relativelocation_y -175.0 _newtrack_0)) false false))
    (:`Finished`
      (`KismetSystemLibrary.Delay` 0.2)
      (`self.K2_DestroyActor`))))

(event `self.Cube.OnComponentBeginOverlap`
  (params (OverlappedComponent :type "PrimitiveComponent Object Reference") (OtherActor :type "Actor Object Reference") (OtherComp :type "PrimitiveComponent Object Reference") (OtherBodyIndex :type Integer) (bFromSweep :type Boolean) (SweepResult :type "HitResult Structure (by ref)"))
  (bind _asbp_top_down_character (cast `/Game/TopDown/Blueprints/BP_TopDownCharacter` OtherActor))
  (if (not (`/Game/TopDown/Blueprints/BP_TopDownCharacter.Invulnerable` _asbp_top_down_character))
    (`GameplayStatics.ApplyDamage` OtherActor 1.0)))

(fn `UserConstructionScript`)