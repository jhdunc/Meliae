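; Explosion hazard for the flying miniboss attack, spawned as a damaging sphere.
; On BeginPlay a timeline scales the sphere up over time.
; Overlapping the top-down player character deals damage unless that character is invulnerable.
; Explosion Niagara effect nodes exist but are disconnected.
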(event `self.ReceiveBeginPlay`
  (bind (_direction _newtrack_2) (`Timeline|Boom Go Big`)
    (:`Update`
      (`SceneComponent.SetRelativeScale3D` (`self.Sphere`) _newtrack_2))))

(event `self.ReceiveActorBeginOverlap`
  (params (OtherActor :type "Actor Object Reference"))
  (bind _asbp_top_down_character (cast `/Game/TopDown/Blueprints/BP_TopDownCharacter` OtherActor))
  (if (not (`/Game/TopDown/Blueprints/BP_TopDownCharacter.Invulnerable` _asbp_top_down_character))
    (`GameplayStatics.ApplyDamage` _asbp_top_down_character 1.0)))

(fn `UserConstructionScript`)