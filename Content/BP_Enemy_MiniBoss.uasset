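; Miniboss enemy for a top-down game that cycles through attacks, mostly advancing with random skips or step-backs.
; Attacks include homing volleys, a booster shot, chasing swipes and spawning minions while repositioning.
; A flying phase lifts the mesh on a timeline, rains telegraphed projectiles by timer, then lands with a radial burst.
; Damage updates health and may drop pickups, with BP_GameManager tracking enemy totals and Tick refreshing the health bar.
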(event `self.ReceiveBeginPlay`
  (bind (_returnvalue_x _returnvalue_y _returnvalue_z) (`KismetMathLibrary.BreakVector` (`self.K2_GetActorLocation`)))
  (bind _as_bp_top_down_character (`self.As BP Top Down Character`))
  (bind _gamemanager (`self.GameManager`))
  (bind _asbp_top_down_character (cast `/Game/TopDown/Blueprints/BP_TopDownCharacter` (`GameplayStatics.GetPlayerCharacter` 0)))
  (set `self.As BP Top Down Character` _asbp_top_down_character)
  (bind _returnvalue (`GameplayStatics.GetActorOfClass` "/Game/TopDown/Blueprints/BP_GameManager.BP_GameManager_C"))
  (set `self.GameManager` _returnvalue)
  (set `/Game/TopDown/Blueprints/BP_TopDownCharacter.EnemyCounter` (+ (`/Game/TopDown/Blueprints/BP_TopDownCharacter.EnemyCounter` _as_bp_top_down_character) 1) _as_bp_top_down_character)
  (`/Game/TopDown/Blueprints/BP_GameManager.SpawnUpdate` _gamemanager (`KismetMathLibrary.FTrunc` (`self.Health`)))
  (`/Game/TopDown/Blueprints/BP_GameManager.UpdateTotalEnemies` _gamemanager true)
  (`self.Attacks`)
  (set `self.Health` (`self.MaxHealth`))
  (`self.Get Random Starting Point`)
  (bind _output_get (set `self.FlyUpZ` (+ _returnvalue_z 900.0)))
  (`KismetSystemLibrary.PrintString` (`KismetStringLibrary.Conv_DoubleToString` _output_get))
  (`KismetSystemLibrary.PrintString` (`KismetStringLibrary.Conv_DoubleToString` _returnvalue_z)))

(event `self.ReceiveTick`
  (params (DeltaSeconds :type "Float (single-precision)"))
  (`self.UpdateHealthbar`))

(event `Attacks`
  (bind _attacknumber (`self.AttackNumber`))
  (`KismetSystemLibrary.Delay` (`KismetMathLibrary.RandomFloatInRange` 0.25 0.35))
  (`KismetSystemLibrary.PrintString` (`KismetStringLibrary.Conv_IntToString` _attacknumber))
  (switch `int` _attacknumber
    (:`Default`
      (`self.Get Random Starting Point`)
      (`self.Attacks`))
    (:`0`
      (set `self.Index` 0)
      (`self.Homing`))
    (:`1`
      (set `self.Index` 0)
      (`|PlayMontage` (`self.Mesh`) "/Game/GameFilesMeliae/Meshes/enemies/animations/AM_Miniboss_bullets.AM_Miniboss_Bullets"
        (:`then`
          (`self.BoosterShot`))))
    (:`2`
      (set `self.Index` 0)
      (`|PlayMontage` (`self.Mesh`) "/Game/GameFilesMeliae/Meshes/enemies/animations/AM_Miniboss_Swipe.AM_Miniboss_Swipe"
        (:`then`
          (`self.Swipe`))))
    (:`3`
      (set `self.Index` 0)
      (`|PlayMontage` (`self.Mesh`) "/Game/GameFilesMeliae/Meshes/enemies/animations/AM_Miniboss_SpawnEnemy.AM_Miniboss_SpawnEnemy"
        (:`then`
          (`self.SpawnSprayers`))))
    (:`4`
      (set `self.Index` 0)
      (`|PlayMontage` (`self.Mesh`)
        (:`then`
          (`self.Fly Up`))))))

(event `Get Random Starting Point`
  (set `self.AttackNumber` (`KismetMathLibrary.RandomIntegerInRange` 0 1)))

(event `SpawnSprayers`
  (bind _randomlocation (`NavigationSystemV1.K2_GetRandomReachablePointInRadius` (`self.K2_GetActorLocation`) 600.0 null null))
  (`KismetSystemLibrary.Delay` 0.33)
  (if (>= (`self.Index`) 2)
    (set `self.Index` 0)
    (`self.CalculateIncrement`)
    (`self.Attacks`)
    (else
      (set `self.RandomMovementLocation` _randomlocation)
      (while (< (`KismetMathLibrary.Vector_Distance` (`self.K2_GetActorLocation` (`GameplayStatics.GetPlayerCharacter` 0)) (`self.RandomMovementLocation`)) 450.0)
        (set `self.RandomMovementLocation` _randomlocation))
      (`KismetSystemLibrary.PrintString` "Moving")
      (`AITask_MoveTo.AIMoveTo` (`AIBlueprintHelperLibrary.GetAIController` self) (`self.RandomMovementLocation`) null 10.0 "Enable" "Enable"
        (:`OnRequestFailed`
          (`KismetSystemLibrary.PrintString` "Req Failed - Miniboss"))
        (:`OnMoveFinished`
          (`KismetSystemLibrary.Delay` 0.33)
          (`|SpawnActorFromClass` "/Game/BP_Enemy_Run_And_Gun.BP_Enemy_Run_And_Gun_C" (`KismetMathLibrary.MakeTransform` (`KismetMathLibrary.RandomPointInBoundingBox` (`self.K2_GetActorLocation`) (200.0 200.0 0.0))) "Undefined" "MultiplyWithRoot" null null)
          (`/Engine/EditorBlueprintResources/StandardMacros.IncrementInt` (`self.Index`)
            (:`  `
              _))))
      (`self.SpawnSprayers`))))

(event `Fly Up`
  (bind (_returnvalue_x _returnvalue_y _returnvalue_z) (`KismetMathLibrary.BreakVector` (`self.K2_GetActorLocation`)))
  (bind _returnvalue (`GameplayStatics.GetActorOfClass` "/Game/TopDown/Blueprints/Terrain/Rooms/Rooms_Children/BP_Room_Start.BP_Room_Start_C"))
  (bind (_returnvalue_x_2 _returnvalue_y_2 _returnvalue_z_2) (`KismetMathLibrary.BreakVector` (`SceneComponent.K2_GetComponentLocation` (`/Game/TopDown/Blueprints/Terrain/Rooms/Rooms_Parent/BP_RoomLayoutStandard.MIDDLE` _returnvalue))))
  (`AITask_MoveTo.AIMoveTo` (`AIBlueprintHelperLibrary.GetAIController` self) (`KismetMathLibrary.MakeVector` _returnvalue_x_2 _returnvalue_y_2 (+ _returnvalue_z_2 50.0)) null 5.0 "Enable" "Enable"
    (:`OnRequestFailed`
      (`KismetSystemLibrary.PrintString` "Req failed - move to center"))
    (:`OnMoveFinished`
      (`self.K2_SetActorRotation` (struct :`Yaw` 180.0))
      (`SkeletalMeshComponent.PlayAnimation` (`self.Mesh`) "/Game/GameFilesMeliae/Characters/Mannequins/Animations/Manny/MM_T_Pose.MM_T_Pose" false)
      (bind (_direction _newtrack_0) (`Timeline|Flying` :!via `PlayFromStart`)
        (:`Update`
          (`SceneComponent.K2_SetWorldLocation` (`self.Mesh`) (`KismetMathLibrary.MakeVector` _returnvalue_x _returnvalue_y (`KismetMathLibrary.Lerp` _returnvalue_z (`self.FlyUpZ`) _newtrack_0)) true false))
        (:`Finished`
          (`KismetSystemLibrary.PrintString` (`KismetStringLibrary.Conv_DoubleToString` _returnvalue_z))
          (`KismetSystemLibrary.K2_SetTimer` null "FlyingAttack" 0.25 true))))))

(event `Fly Down`
  (bind (_returnvalue_x _returnvalue_y _returnvalue_z) (`KismetMathLibrary.BreakVector` (`self.K2_GetActorLocation`)))
  (bind (_returnvalue_x_2 _returnvalue_y_2 _returnvalue_z_2) (`KismetMathLibrary.BreakVector` (`self.K2_GetActorLocation`)))
  (bind (_returnvalue_location _returnvalue_rotation) (`KismetMathLibrary.BreakTransform` (`SceneComponent.K2_GetComponentToWorld` (`self.BulletSpawnPoint`))))
  (`KismetSystemLibrary.Delay` 2.0)
  (`SkeletalMeshComponent.PlayAnimation` (`self.Mesh`) "/Game/GameFilesMeliae/Characters/Mannequins/Animations/Manny/MM_T_Pose.MM_T_Pose" false)
  (bind (_direction _newtrack_0) (`Timeline|Timeline` :!via `PlayFromStart`)
    (:`Update`
      (`SceneComponent.K2_SetWorldLocation` (`self.Mesh`) (`KismetMathLibrary.MakeVector` _returnvalue_x_2 _returnvalue_y_2 (`KismetMathLibrary.Lerp` _returnvalue_z_2 (- (`self.FlyUpZ`) 900.0) _newtrack_0)) true false))
    (:`Finished`
      (`KismetSystemLibrary.PrintString` (`KismetStringLibrary.Conv_DoubleToString` _returnvalue_z))
      (for _index (range 18)
        (`SceneComponent.K2_SetWorldRotation` (`self.SpinTarget`) (`KismetMathLibrary.MakeRotator` 0.0 0.0 (* _index 20)) false false)
        (`|SpawnActorFromClass` "/Game/Projectiles/BP_Enemy_Miniboss_SlamDown_Projectile.BP_Enemy_Miniboss_SlamDown_Projectile_C" (`KismetMathLibrary.MakeTransform` _returnvalue_location _returnvalue_rotation) "Undefined" "MultiplyWithRoot" null null))
      (`SceneComponent.K2_SetRelativeRotation` :`self` (`self.SpinTarget`))
      (`self.CalculateIncrement`)
      (`self.Attacks`))))

(event `CalculateIncrement`
  (if (== (`KismetMathLibrary.RandomIntegerInRange` 1 5) 5)
    (set `self.AttackNumber` (`KismetMathLibrary.Clamp` (- (`self.AttackNumber`) 1) 0 10))
    (elif (== (`KismetMathLibrary.RandomIntegerInRange` 1 4) 4)
      (set `self.AttackNumber` (+ (`self.AttackNumber`) 2))
      (else
        (`/Engine/EditorBlueprintResources/StandardMacros.IncrementInt` (`self.AttackNumber`))))))

(event `self.ReceiveAnyDamage`
  (params (Damage :type "Float (single-precision)") (DamageType :type "DamageType Object Reference") (InstigatedBy :type "Controller Object Reference") (DamageCauser :type "Actor Object Reference"))
  (`NiagaraFunctionLibrary.SpawnSystemAtLocation` "/Game/GameFilesMeliae/VFX/DamageFlash/NG_EnemyDamageParticle.NG_EnemyDamageParticle" (`self.K2_GetActorLocation`))
  (`/Game/TopDown/Blueprints/BP_GameManager.SpawnPickup` (`self.GameManager`) self 2)
  (set `self.Health` (- (`self.Health`) (`KismetMathLibrary.Round` Damage)))
  (`/Game/TopDown/Blueprints/BP_GameManager.SubtractEnemyCurrent` (`self.GameManager`))
  (if (<= (`self.Health`) 0)
    (`self.K2_DestroyActor`)))

(event `Swipe`
  (bind _charactermovement (`self.CharacterMovement`))
  (`KismetSystemLibrary.Delay` 0.45)
  (if (>= (`self.Index`) 3)
    (set `CharacterMovementComponent.MaxWalkSpeed` 600.0 _charactermovement)
    (`self.CalculateIncrement`)
    (`self.Attacks`)
    (else
      (set `CharacterMovementComponent.MaxWalkSpeed` 850.0 _charactermovement)
      (`AITask_MoveTo.AIMoveTo` (`AIBlueprintHelperLibrary.GetAIController` self) (0.0 0.0 0.0) (`GameplayStatics.GetPlayerCharacter` 0) 50.0 "Enable" "Enable"
        (:`OnRequestFailed`
          (`KismetSystemLibrary.PrintString` "Req Failed - Move to Player Miniboss"))
        (:`OnMoveFinished`
          (`SkeletalMeshComponent.PlayAnimation` (`self.Mesh`) "/Game/GameFilesMeliae/Characters/Mannequins/Animations/Manny/MM_T_Pose.MM_T_Pose" false)
          (`KismetSystemLibrary.Delay` 0.28)
          (`|SpawnActorFromClass` "/Game/Projectiles/BP_Enemy_Miniboss_Swipe_Hitbox.BP_Enemy_Miniboss_Swipe_Hitbox_C" (`SceneComponent.K2_GetComponentToWorld` (`self.BulletSpawnPoint`)) "Undefined" "MultiplyWithRoot" null null)
          (`/Engine/EditorBlueprintResources/StandardMacros.IncrementInt` (`self.Index`)
            (:`  `
              (`self.Swipe`))))))))

(event `self.ReceiveDestroyed`
  (`/Game/TopDown/Blueprints/BP_GameManager.UpdateTotalEnemies` (`self.GameManager`) false))

(event `Homing`
  (bind _index (`self.Index`))
  (`/Engine/EditorBlueprintResources/StandardMacros.IncrementInt` (`self.Index`)
    (:`  `
      (`|ExecutionSequence`
        (:`then_0`
          (`|SpawnActorFromClass` "/Game/BP_Miniboss_Homing_Projectile.BP_Miniboss_Homing_Projectile_C" (`SceneComponent.K2_GetComponentToWorld` (`self.HomingSpawnPoint1`)) "Undefined" "MultiplyWithRoot" null null))
        (:`then_1`
          (`|SpawnActorFromClass` "/Game/BP_Miniboss_Homing_Projectile.BP_Miniboss_Homing_Projectile_C" (`SceneComponent.K2_GetComponentToWorld` (`self.HomingSpawnPoint2`)) "Undefined" "MultiplyWithRoot" null null)
          (`KismetSystemLibrary.PrintString` (`KismetStringLibrary.Conv_IntToString` _index))
          (if (>= _index 3)
            (`self.CalculateIncrement`)
            (`self.Attacks`)
            (else
              (`KismetSystemLibrary.Delay` 0.25)
              (`self.Homing`))))))))

(event `BoosterShot`
  (bind (_rotationrate_roll _rotationrate_pitch _rotationrate_yaw) (`KismetMathLibrary.BreakRotator` (`CharacterMovementComponent.RotationRate` (`self.CharacterMovement`))))
  (`self.K2_SetActorRotation` (`KismetMathLibrary.RInterpTo_Constant` (`self.K2_GetActorRotation`) (`KismetMathLibrary.FindLookAtRotation` (`self.K2_GetActorLocation`) (`self.K2_GetActorLocation` (`GameplayStatics.GetPlayerCharacter` 0))) (`GameplayStatics.GetWorldDeltaSeconds`) _rotationrate_yaw))
  (`KismetSystemLibrary.Delay` 0.4)
  (`|SpawnActorFromClass` "/Game/Projectiles/BP_Miniboss_BoosterStage1_Projectile.BP_Miniboss_BoosterStage1_Projectile_C" (`SceneComponent.K2_GetComponentToWorld` (`self.BulletSpawnPoint`)) "Undefined" "MultiplyWithRoot" null null)
  (`self.CalculateIncrement`)
  (`self.Attacks`))

(fn `FlyingAttack`
  (bind (_random_location_x _random_location_y _random_location_z) (`KismetMathLibrary.BreakVector` (`self.Random Location`)))
  (bind (_returnvalue_x _returnvalue_y _returnvalue_z) (`KismetMathLibrary.BreakVector` (`KismetMathLibrary.RandomPointInBoundingBox` (`SceneComponent.K2_GetComponentLocation` (`self.Mesh`)) (850.0 850.0 0.0))))
  (`/Engine/EditorBlueprintResources/StandardMacros.IncrementInt` (`self.Index`)
    (:`  `
      (bind _output_get (set `self.Random Location` (`KismetMathLibrary.MakeVector` _returnvalue_x _returnvalue_y (- _returnvalue_z 350.0))))
      (bind _returnvalue (`|SpawnActorFromClass` "/Game/Projectiles/BP_Enemy_Miniboss_Projectile_Drop.BP_Enemy_Miniboss_Projectile_Drop_C" (`KismetMathLibrary.MakeTransform` _output_get) "AdjustIfPossibleButDontSpawnIfColliding" "MultiplyWithRoot" null null))
      (`|SpawnActorFromClass` "/Game/Projectiles/BP_Enemy_Miniboss_FlyingAttack_Indicator.BP_Enemy_Miniboss_FlyingAttack_Indicator_C" (`KismetMathLibrary.MakeTransform` (`KismetMathLibrary.MakeVector` _random_location_x _random_location_y (- _random_location_z 230.0))) "Undefined" "MultiplyWithRoot" null null)
      (`KismetSystemLibrary.PrintString` (`KismetStringLibrary.Conv_VectorToString` (`self.K2_GetActorLocation` _returnvalue)))
      (if (>= (`self.Index`) 36)
        (`KismetSystemLibrary.K2_ClearTimer` null "FlyingAttack")
        (set `self.Index` 0)
        (`self.Fly Down`)))))

(fn `UpdateHealthbar`
  (bind _aswb_enemy_health (cast `/Game/GameFilesMeliae/UI/WB_EnemyHealth` (`WidgetComponent.GetUserWidgetObject` (`self.HealthBarWidget`))))
  (set `/Game/GameFilesMeliae/UI/WB_EnemyHealth.Health` (/ (`self.Health`) (`self.MaxHealth`)) _aswb_enemy_health)
  (return))

(fn `UserConstructionScript`)