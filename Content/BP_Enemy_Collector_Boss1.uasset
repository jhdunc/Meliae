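; Collector boss enemy that turns to face the player, shows a health bar, reports to BP_GameManager and displays the win screen when destroyed.
; Attacks cycles through five patterns by AttackCounter: spinning bullets, log walls, aimed spread bursts, summoned adds and bullet walls.
; Each pattern is a looping timer-by-name sharing an Index counter; LoopAmount or BurstFire's own check clears it and re-enters Attacks.
; QuickShot is defined but outside the cycle.
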(event `self.ReceiveTick`
  (params (DeltaSeconds :type "Float (single-precision)"))
  (`self.UpdateHealthbar`)
  ;[0.8549 0.2902 0.05098] Make Our Boy Spin
  (`self.K2_SetActorRotation` (`KismetMathLibrary.MakeRotator` 0.0 0.0 (.yaw (.rotation (`KismetAnimationLibrary.K2_LookAt` (`self.GetTransform`) (`self.K2_GetActorLocation` (`self.PlayerRef`)) (1.0 0.0 0.0)))))))

(event `self.ReceiveBeginPlay`
  (set `self.Health` (`self.MaxHealth`))
  (bind _returnvalue (`GameplayStatics.GetActorOfClass` "/Game/TopDown/Blueprints/BP_GameManager.BP_GameManager_C"))
  (bind _output_get (set `self.GameManager` _returnvalue))
  (`/Game/TopDown/Blueprints/BP_GameManager.SpawnUpdate` _output_get (`KismetMathLibrary.FTrunc` (`self.Health`)))
  (`/Game/TopDown/Blueprints/BP_GameManager.UpdateTotalEnemies` _output_get true)
  (bind _asbp_top_down_character (cast `/Game/TopDown/Blueprints/BP_TopDownCharacter` (`GameplayStatics.GetPlayerCharacter` 0)))
  (set `self.PlayerRef` _asbp_top_down_character)
  (`self.Attacks`))

(event `Attacks`
  (bind _boss (`self.Boss`))
  (bind _boss_2 (`self.Boss`))
  (if (not (== (`self.AttackCounter`) 2))
    (`SkeletalMeshComponent.PlayAnimation` (`self.Boss`) "/Game/GameFilesMeliae/Meshes/Boss/Boss_Anim_Armature_idle.Boss_Anim_Armature_idle" false))
  (`KismetSystemLibrary.Delay` (`KismetMathLibrary.RandomFloatInRange` 0.6 0.75))
  (switch `int` (`self.AttackCounter`)
    (:`Default`
      (set `self.AttackCounter` 0)
      (`self.Attacks`))
    (:`0`
      (`SkeletalMeshComponent.PlayAnimation` _boss_2 "/Game/GameFilesMeliae/Meshes/Boss/Boss_Anim_Armature_Spin_to_shoot_bullets.Boss_Anim_Armature_Spin_to_shoot_bullets" true)
      (`KismetSystemLibrary.K2_SetTimer` null "Spin" (`self.DelayBetweenBulletsSpin`) true))
    (:`1`
      (`SkeletalMeshComponent.PlayAnimation` _boss_2 "/Game/GameFilesMeliae/Meshes/Boss/Boss_Anim_Armature_Placing_log.Boss_Anim_Armature_Placing_log" true)
      (`KismetSystemLibrary.K2_SetTimer` null "LogWalls" (`self.DelayBetweenLogSpawn`) true))
    (:`2`
      (`SkeletalMeshComponent.PlayAnimation` _boss "/Game/GameFilesMeliae/Meshes/Boss/Boss_Anim_Armature_Shoot_in_spread_and_plus_pattern.Boss_Anim_Armature_Shoot_in_spread_and_plus_pattern" true)
      (`KismetSystemLibrary.K2_SetTimer` null "BurstFire" (`self.DelayBetweenBurstFire`) true))
    (:`3`
      (`SkeletalMeshComponent.PlayAnimation` _boss "/Game/GameFilesMeliae/Meshes/Boss/Boss_Anim_Armature_Summoning_enemies.Boss_Anim_Armature_Summoning_enemies" true)
      (`KismetSystemLibrary.Delay` 1.5)
      (`KismetSystemLibrary.K2_SetTimer` null "SpawnAdds" 0.02 true))
    (:`4`
      (`SkeletalMeshComponent.PlayAnimation` _boss "/Game/GameFilesMeliae/Meshes/Boss/Boss_Anim_Armature_Shoot_in_spread_and_plus_pattern.Boss_Anim_Armature_Shoot_in_spread_and_plus_pattern" true)
      (`KismetSystemLibrary.K2_SetTimer` null "BulletWall" 0.05 true))))

(event `self.ReceiveAnyDamage`
  (params (Damage :type "Float (single-precision)") (DamageType :type "DamageType Object Reference") (InstigatedBy :type "Controller Object Reference") (DamageCauser :type "Actor Object Reference"))
  (bind _gamemanager (`self.GameManager`))
  ;[0 1 0.9622] wow, the damage particle works
  (`NiagaraFunctionLibrary.SpawnSystemAtLocation` "/Game/GameFilesMeliae/VFX/DamageFlash/NG_EnemyDamageParticle.NG_EnemyDamageParticle" (`self.K2_GetActorLocation`) (struct) (2.0 2.0 2.0))
  (set `self.Health` (- (`self.Health`) (`KismetMathLibrary.Round` Damage)))
  (`/Game/TopDown/Blueprints/BP_GameManager.SpawnPickup` _gamemanager null 5)
  (`/Game/TopDown/Blueprints/BP_GameManager.SubtractEnemyCurrent` _gamemanager)
  (if (<= (`self.Health`) 0.0)
    (`NiagaraFunctionLibrary.SpawnSystemAtLocation` "/Game/GameFilesMeliae/VFX/DamageFlash/NG_BossDeath1.NG_BossDeath1" (`self.K2_GetActorLocation`))
    (`self.K2_DestroyActor`)))

(event `self.ReceiveDestroyed`
  ;[0.8549 0.2902 0.05098] Countdown for All Enemies Dead condition
  (`/Game/TopDown/Blueprints/BP_GameManager.UpdateTotalEnemies` (`self.GameManager`) false)
  (bind _returnvalue (`|CreateWidget` "/Game/GameFilesMeliae/UI/WB_Game_OverWin.WB_Game_OverWin_C" (`GameplayStatics.GetPlayerController` 0)))
  (`UserWidget.AddToViewport` _returnvalue 0))

(fn `BulletWall`
  (bind _index (`self.Index`))
  (bind _returnvalue_location (`KismetMathLibrary.BreakTransform` (`SceneComponent.K2_GetComponentToWorld` (`self.BulletSpawnPoint`))))
  (for _index_2 (range 3)
    (`SceneComponent.K2_SetWorldRotation` (`self.SpinTarget`) (`KismetMathLibrary.MakeRotator` 0.0 0.0 (`KismetMathLibrary.Conv_IntToDouble` (* _index_2 180))) false false)
    (`|SpawnActorFromClass` "/Game/Projectiles/BP_Enemy_Projectile_Collector_Boss_Wall.BP_Enemy_Projectile_Collector_Boss_Wall_C" (`KismetMathLibrary.MakeTransform` _returnvalue_location) "Undefined" "MultiplyWithRoot" null null))
  (`SceneComponent.K2_SetRelativeRotation` :`self` (`self.SpinTarget`))
  (`SceneComponent.K2_SetRelativeLocation` (`self.BulletSpawnPoint`) (`KismetMathLibrary.MakeVector` (`KismetMathLibrary.Conv_IntToDouble` (+ (* _index 50) 75)) 0.0 -45.0) false false)
  (bind _result (`/Engine/EditorBlueprintResources/StandardMacros.IncrementInt` _index)
    (:`  `
      (if (>= _result 25)
        (`SceneComponent.K2_SetRelativeLocation` (`self.BulletSpawnPoint`) (75.0 0.0 -45.0) false false)
        (`self.LoopAmount` 50 "BulletWall")))))

(fn `BurstFire`
  (bind (_returnvalue_location _returnvalue_rotation) (`KismetMathLibrary.BreakTransform` (`SceneComponent.K2_GetComponentToWorld` (`self.BulletSpawnPoint`))))
  (bind (_returnvalue_roll _returnvalue_pitch _returnvalue_yaw) (`KismetMathLibrary.BreakRotator` (`KismetMathLibrary.FindLookAtRotation` (`self.K2_GetActorLocation`) (`self.K2_GetActorLocation` (`GameplayStatics.GetPlayerCharacter` 0)))))
  (`|ExecutionSequence`
    (:`then_0`
      (`/Engine/EditorBlueprintResources/StandardMacros.DoOnce` false :!label _label
        (:`Completed`
          (`SkeletalMeshComponent.PlayAnimation` (`self.Mesh`) "/Game/GameFilesMeliae/Meshes/Boss/Boss_Anim_Armature_Shoot_in_spread_and_plus_pattern.Boss_Anim_Armature_Shoot_in_spread_and_plus_pattern" true))))
    (:`then_1`
      (`/Engine/EditorBlueprintResources/StandardMacros.IncrementInt` (`self.Index`)
        (:`  `
          (`SceneComponent.K2_SetWorldRotation` (`self.SpinTarget`) (`KismetMathLibrary.MakeRotator` 0.0 0.0 _returnvalue_yaw) false false)
          (for _index (range -2 3)
            (bind _returnvalue (`|SpawnActorFromClass` "/Game/Projectiles/BP_Enemy_Projectile_Collector_Boss_Burst.BP_Enemy_Projectile_Collector_Boss_Burst_C" (`KismetMathLibrary.MakeTransform` _returnvalue_location _returnvalue_rotation) "Undefined" "MultiplyWithRoot" null null))
            (`ProjectileMovementComponent.SetVelocityInLocalSpace` (`/Game/Projectiles/BP_Enemy_Projectile_Collector_Boss_Burst.ProjectileMovement` _returnvalue) (`KismetMathLibrary.MakeVector` 1600.0 (* _index 200))))
          (if (== (`KismetMathLibrary.FMod` (`KismetMathLibrary.Conv_IntToDouble` (`self.Index`)) 5.0) 0.0)
            (`KismetSystemLibrary.K2_ClearTimer` null "BurstFire")
            (if (== (`self.Index`) 15)
              (set `self.Index` 0)
              (`/Engine/EditorBlueprintResources/StandardMacros.IncrementInt` (`self.AttackCounter`)
                (:`  `
                  (`SkeletalMeshComponent.PlayAnimation` (`self.Boss`) "/Game/GameFilesMeliae/Meshes/Boss/Boss_Anim_Armature_idle.Boss_Anim_Armature_idle" true)
                  (`|ExecutionSequence`
                    (:`then_0`
                      (goto _label :!via `Reset`))
                    (:`then_1`
                      _)))))
            (`self.Attacks`)))))))

(fn `LogWalls`
  (bind (_returnvalue_roll _returnvalue_pitch) (`KismetMathLibrary.BreakRotator` (`SceneComponent.K2_GetComponentRotation` (`self.SpinTarget`))))
  (bind (_returnvalue_location _returnvalue_rotation) (`KismetMathLibrary.BreakTransform` (`SceneComponent.K2_GetComponentToWorld` (`self.LogSpawnPoint`))))
  (`/Engine/EditorBlueprintResources/StandardMacros.IncrementInt` (`self.Index`)
    (:`  `
      (`SceneComponent.K2_SetRelativeRotation` (`self.SpinTarget`) (`KismetMathLibrary.MakeRotator` _returnvalue_roll _returnvalue_pitch (`KismetMathLibrary.Conv_IntToDouble` (* (`self.Index`) 90))) false false)
      (`|SpawnActorFromClass` "/Game/TopDown/Blueprints/Greybox/BP_Enemy_Crafter_Log_Pile.BP_Enemy_Crafter_Log_Pile_C" (`KismetMathLibrary.MakeTransform` _returnvalue_location _returnvalue_rotation) "AdjustIfPossibleButAlwaysSpawn" "MultiplyWithRoot" null null)
      (`self.LoopAmount` 4 "LogWalls"))))

(fn `QuickShot`
  (bind (_returnvalue_location _returnvalue_rotation) (`KismetMathLibrary.BreakTransform` (`SceneComponent.K2_GetComponentToWorld` (`self.BulletSpawnPoint`))))
  (bind (_returnvalue_roll _returnvalue_pitch _returnvalue_yaw) (`KismetMathLibrary.BreakRotator` (`KismetMathLibrary.FindLookAtRotation` (`self.K2_GetActorLocation`) (`self.K2_GetActorLocation` (`GameplayStatics.GetPlayerCharacter` 0)))))
  (`SceneComponent.K2_SetRelativeRotation` (`self.SpinTarget`) (`KismetMathLibrary.MakeRotator` 0.0 0.0 _returnvalue_yaw) false false)
  (bind _returnvalue (`|SpawnActorFromClass` "/Game/Projectiles/BP_Enemy_Projectile_Collector_Boss_Burst.BP_Enemy_Projectile_Collector_Boss_Burst_C" (`KismetMathLibrary.MakeTransform` _returnvalue_location _returnvalue_rotation) "Undefined" "MultiplyWithRoot" null null))
  (bind _projectilemovement (`/Game/Projectiles/BP_Enemy_Projectile_Collector_Boss_Burst.ProjectileMovement` _returnvalue))
  (set `ProjectileMovementComponent.InitialSpeed` 1650.0 _projectilemovement)
  (set `ProjectileMovementComponent.MaxSpeed` 1650.0 _projectilemovement))

(fn `SpawnAdds`
  (bind (_random_location_x _random_location_y _random_location_z) (`KismetMathLibrary.BreakVector` (`self.Random Location`)))
  (bind _randomlocation (`NavigationSystemV1.K2_GetRandomReachablePointInRadius` (`self.K2_GetActorLocation`) 300.0 null null))
  (`/Engine/EditorBlueprintResources/StandardMacros.IncrementInt` (`self.Index`)
    (:`  `
      (set `self.Random Location` _randomlocation)
      (while (< (`KismetMathLibrary.Vector_Distance` (`self.K2_GetActorLocation` (`GameplayStatics.GetPlayerCharacter` 0)) (`self.Random Location`)) 100.0)
        (set `self.Random Location` _randomlocation))
      (bind _returnvalue (`|SpawnActorFromClass` "/Game/BP_Enemy_Run_And_Gun.BP_Enemy_Run_And_Gun_C" (`KismetMathLibrary.MakeTransform` (`KismetMathLibrary.MakeVector` _random_location_x _random_location_y (- _random_location_z 20.0))) "AdjustIfPossibleButDontSpawnIfColliding" "MultiplyWithRoot" null null))
      (`NiagaraFunctionLibrary.SpawnSystemAtLocation` "/Game/GameFilesMeliae/VFX/Bullets/NG_AddsSpawn.NG_AddsSpawn" (`self.K2_GetActorLocation` _returnvalue))
      (`self.LoopAmount` 2 "SpawnAdds"))))

(fn `Spin`
  (bind (_returnvalue_location _returnvalue_rotation) (`KismetMathLibrary.BreakTransform` (`SceneComponent.K2_GetComponentToWorld` (`self.BulletSpawnPoint`))))
  (bind (_returnvalue_roll _returnvalue_pitch) (`KismetMathLibrary.BreakRotator` (`SceneComponent.K2_GetComponentRotation` (`self.SpinTarget`))))
  (`|ExecutionSequence`
    (:`then_1`
      (`/Engine/EditorBlueprintResources/StandardMacros.IncrementInt` (`self.Index`)
        (:`  `
          (`SceneComponent.K2_SetRelativeRotation` (`self.SpinTarget`) (`KismetMathLibrary.MakeRotator` _returnvalue_roll _returnvalue_pitch (`KismetMathLibrary.Conv_IntToDouble` (* (`self.Index`) 12))) false false)
          (`|SpawnActorFromClass` "/Game/Projectiles/BP_Enemy_Projectile_Collector_Boss_Spin.BP_Enemy_Projectile_Collector_Boss_Spin_C" (`KismetMathLibrary.MakeTransform` _returnvalue_location _returnvalue_rotation) "Undefined" "MultiplyWithRoot" null null)
          (`self.LoopAmount` 90 "Spin"))))))

(fn `UpdateHealthbar`
  (bind _aswb_enemy_health (cast `/Game/GameFilesMeliae/UI/WB_EnemyHealth` (`WidgetComponent.GetUserWidgetObject` (`self.HealthBarWidget`))))
  (set `/Game/GameFilesMeliae/UI/WB_EnemyHealth.Health` (/ (`self.Health`) (`self.MaxHealth`)) _aswb_enemy_health)
  (return))

(fn `UserConstructionScript`)