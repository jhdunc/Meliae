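; BP_Enemy_Swarmer is a melee enemy that chases and damages the top-down player character.
; A self-repeating Rotate event with a short delay turns it on yaw toward the player from BeginPlay.
; Entering Sphere1 activates it after a delay, and Tick then pushes it forward through FloatingPawnMovement.
; Cube overlaps toggle contact damage, with Delay nodes on Tick throttling both damage and movement input.
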(event `self.Sphere1.OnComponentBeginOverlap`
  (params (OverlappedComponent :type "PrimitiveComponent Object Reference") (OtherActor :type "Actor Object Reference") (OtherComp :type "PrimitiveComponent Object Reference") (OtherBodyIndex :type Integer) (bFromSweep :type Boolean) (SweepResult :type "HitResult Structure (by ref)"))
  (cast `/Game/TopDown/Blueprints/BP_TopDownCharacter` OtherActor)
  (`KismetSystemLibrary.Delay` 0.5)
  (set `self.Active` true))

(event `self.ReceiveTick`
  (params (DeltaSeconds :type "Float (single-precision)"))
  (`|ExecutionSequence`
    (:`then_0`
      (if (`self.Active`)
        (`KismetSystemLibrary.Delay` 0.0175)
        (`PawnMovementComponent.AddInputVector` (`self.FloatingPawnMovement`) (`KismetMathLibrary.GetForwardVector` (`self.K2_GetActorRotation`)) false)))
    (:`then_1`
      (if (`self.Overlapping`)
        (`KismetSystemLibrary.Delay` 1.0)
        (`GameplayStatics.ApplyDamage` (`self.As BP Top Down Character`) (`self.Base Damage`))))))

(event `self.ReceiveBeginPlay`
  (bind _asbp_top_down_character (cast `/Game/TopDown/Blueprints/BP_TopDownCharacter` (`GameplayStatics.GetPlayerCharacter` 0)))
  (set `self.As BP Top Down Character` _asbp_top_down_character)
  (`self.Rotate`))

(event `Rotate`
  (`self.K2_SetActorRotation` (`KismetMathLibrary.MakeRotator` 0.0 0.0 (.yaw (`KismetMathLibrary.RInterpTo` (`self.K2_GetActorRotation`) (`KismetMathLibrary.FindLookAtRotation` (`self.K2_GetActorLocation`) (`self.K2_GetActorLocation` (`self.As BP Top Down Character`))) (`GameplayStatics.GetWorldDeltaSeconds`) 25.0))))
  (`KismetSystemLibrary.Delay` 0.01)
  (`self.Rotate`))

(event `self.Cube.OnComponentBeginOverlap`
  (params (OverlappedComponent :type "PrimitiveComponent Object Reference") (OtherActor :type "Actor Object Reference") (OtherComp :type "PrimitiveComponent Object Reference") (OtherBodyIndex :type Integer) (bFromSweep :type Boolean) (SweepResult :type "HitResult Structure (by ref)"))
  (cast `/Game/TopDown/Blueprints/BP_TopDownCharacter` OtherActor)
  (set `self.Overlapping` true))

(event `self.Cube.OnComponentEndOverlap`
  (params (OverlappedComponent :type "PrimitiveComponent Object Reference") (OtherActor :type "Actor Object Reference") (OtherComp :type "PrimitiveComponent Object Reference") (OtherBodyIndex :type Integer))
  (cast `/Game/TopDown/Blueprints/BP_TopDownCharacter` OtherActor)
  (set `self.Overlapping` false))

(fn `UserConstructionScript`)