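; Spawner actor that places enemies at its tagged spawn points when play begins.
; BeginPlay gathers static mesh components tagged "Spawnpoint" and pairs each by index with an EnemyClasses entry.
; A switch on that entry spawns the Run And Gun enemy for Sprayer or the Heavy enemy at the point's location and rotation.
; The Lobber branch has no class assigned, and unmatched entries print a wrong-name warning.
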(event `self.ReceiveBeginPlay`
  (bind _output_get (set `self.Spawnpoints` (`self.GetComponentsByTag` "/Script/Engine.StaticMeshComponent" "Spawnpoint")))
  (for (_array_element _array_index) _output_get
    (switch `string` (`|GetArrayItem` (`self.EnemyClasses`) _array_index)
      (:`Default`
        (`KismetSystemLibrary.PrintString` "Typed Wrong Name"))
      (:`Sprayer`
        (bind (_returnvalue_location _returnvalue_rotation) (`KismetMathLibrary.BreakTransform` (`SceneComponent.K2_GetComponentToWorld` _array_element)))
        (bind _returnvalue (`KismetMathLibrary.MakeTransform` _returnvalue_location _returnvalue_rotation))
        (`|SpawnActorFromClass` "/Game/BP_Enemy_Run_And_Gun.BP_Enemy_Run_And_Gun_C" _returnvalue "Undefined" "MultiplyWithRoot" null null))
      (:`Lobber`
        (`|SpawnActorFromClass` "/Game/BP_Enemy_Lobber.BP_Enemy_Lobber_C" _returnvalue "Undefined" "MultiplyWithRoot" null null))
      (:`Heavy`
        (`|SpawnActorFromClass` "/Game/BP_Enemy_Heavy.BP_Enemy_Heavy_C" _returnvalue "Undefined" "MultiplyWithRoot" null null)))))

(fn `UserConstructionScript`)